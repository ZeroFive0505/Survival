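; Bouncing grenade launcher projectile that explodes on a per-tick sphere trace hit or after reaching its bounce limit.
; On authority, it gathers living characters in the explosion radius, applies a GAS damage effect container and pushes those killed with radial force.
; Cosmetic gameplay cues run locally through player 0's ability system: fire for non-local shooters, impact on EndPlay.
; EndPlay also shakes the instigator's camera when nearby.
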(event `self.ReceiveBeginPlay`
  (bind _asbp_survivor (cast `/Game/Survival/Blueprints/Characters/BP_Survivor` (`self.GetInstigator`)))
  (bind _asgsability_system_component (cast `GSAbilitySystemComponent` (`AbilitySystemBlueprintLibrary.GetAbilitySystemComponent` (`Controller.PlayerState` (`GameplayStatics.GetPlayerController` 0)))))
  (set `self.ASC` _asgsability_system_component)
  (if (not (`Pawn.IsLocallyControlled` _asbp_survivor))
    (`GSAbilitySystemComponent.ExecuteGameplayCueLocal` (`self.ASC`) (struct :`TagName` "GameplayCue.Weapon.RocketLauncher.Fire") (`AbilitySystemBlueprintLibrary.MakeGameplayCueParameters` 0.0 0.0 (struct) (struct) (struct) (struct) (struct) (`self.K2_GetActorLocation`) (`KismetMathLibrary.GetForwardVector` (`self.K2_GetActorRotation`)) _asbp_survivor))))

(event `self.ReceiveTick`
  (params (DeltaSeconds :type "Float (single-precision)"))
  (bind _returnvalue (`self.K2_GetActorLocation`))
  (bind _returnvalue_2 (`self.K2_GetActorLocation`))
  (bind (_outhit _returnvalue_3) (`KismetSystemLibrary.SphereTraceSingle` :`Start` _returnvalue_2 :`End` _returnvalue_2 :`Radius` 16.0 :`TraceChannel` "TraceTypeQuery3" :`bTraceComplex` true :`DrawDebugType` "ForOneFrame"))
  (if _returnvalue_3
    (`/Engine/EditorBlueprintResources/ActorMacros.Switch Has Authority`
      (:`Authority`
        (bind _outhits (`KismetSystemLibrary.SphereTraceMultiForObjects` _returnvalue (+ _returnvalue 0.01) (`self.ExplosionRadius`) (`|MakeArray` "ObjectTypeQuery3" "ObjectTypeQuery12" :!type "EObjectTypeQuery Enum")))
        (for _array_element _outhits
          (bind _asgscharacter (cast `GSCharacter` (`.HitActor` (`GameplayStatics.BreakHitResult` _array_element))))
          (if (`GSCharacter.IsAlive` _asgscharacter)
            (`KismetArrayLibrary.Array_AddUnique` (`self.HitTargets`) _asgscharacter)))
        (`GSBlueprintFunctionLibrary.AddTargetsToEffectContainerSpec` :`ContainerSpec` (`self.DamageEffectContainerSpec`) :`TargetActors` (`self.HitTargets`))
        (`GSBlueprintFunctionLibrary.ApplyExternalEffectContainerSpec` (`self.DamageEffectContainerSpec`))
        (`|ExecutionSequence`
          (:`then_0`
            (for _array_element_2 (`self.HitTargets`)
              (if (not (`GSCharacter.IsAlive` _array_element_2))
                (`PrimitiveComponent.AddRadialForce` (`Character.Mesh` _array_element_2) (`self.K2_GetActorLocation`) (`self.ExplosionRadius`) (`self.ForceAmount`) "RIF_Constant" true))))
          (:`then_1`
            (`self.K2_DestroyActor`))))
      (:`Remote`
        (`self.K2_DestroyActor`)))))

(event `self.StaticMesh.OnComponentHit`
  (params (HitComponent :type "PrimitiveComponent Object Reference") (OtherActor :type "Actor Object Reference") (OtherComp :type "PrimitiveComponent Object Reference") (NormalImpulse :type "Vector Structure") (Hit :type "HitResult Structure (by ref)"))
  (bind _returnvalue (`self.K2_GetActorLocation`))
  (`/Engine/EditorBlueprintResources/StandardMacros.IncrementInt` (`self.CurrentBounce`)
    (:`  `
      (if (>= (`self.CurrentBounce`) (`self.MaxBounce`))
        (`/Engine/EditorBlueprintResources/ActorMacros.Switch Has Authority`
          (:`Authority`
            (bind _outhits (`KismetSystemLibrary.SphereTraceMultiForObjects` _returnvalue (+ _returnvalue 0.01) (`self.ExplosionRadius`) (`|MakeArray` "ObjectTypeQuery3" "ObjectTypeQuery12" :!type "EObjectTypeQuery Enum")))
            (for _array_element _outhits
              (bind _asgscharacter (cast `GSCharacter` (`.HitActor` (`GameplayStatics.BreakHitResult` _array_element))))
              (if (`GSCharacter.IsAlive` _asgscharacter)
                (`KismetArrayLibrary.Array_AddUnique` (`self.HitTargets`) _asgscharacter)))
            (`GSBlueprintFunctionLibrary.AddTargetsToEffectContainerSpec` :`ContainerSpec` (`self.DamageEffectContainerSpec`) :`TargetActors` (`self.HitTargets`))
            (`GSBlueprintFunctionLibrary.ApplyExternalEffectContainerSpec` (`self.DamageEffectContainerSpec`))
            (`|ExecutionSequence`
              (:`then_0`
                (for _array_element_2 (`self.HitTargets`)
                  (if (not (`GSCharacter.IsAlive` _array_element_2))
                    (`PrimitiveComponent.AddRadialForce` (`Character.Mesh` _array_element_2) (`self.K2_GetActorLocation`) (`self.ExplosionRadius`) (`self.ForceAmount`) "RIF_Constant" true))))
              (:`then_1`
                (`self.K2_DestroyActor`))))
          (:`Remote`
            (`self.K2_DestroyActor`)))
        (else
          (`GameplayStatics.PlaySoundAtLocation` "/Game/MilitaryWeapDark/Sound/GrenadeLauncher/GrenadeLauncher_Bounce_Cue.GrenadeLauncher_Bounce_Cue" (`self.K2_GetActorLocation`) (struct) 1.0 1.0 0.0 null null null null))))))

(event `self.ReceiveEndPlay`
  (params (EndPlayReason :type "EEndPlayReason Enum" :default "Destroyed"))
  (bind _asc (`self.ASC`)
    (:`then`
      (`GSAbilitySystemComponent.ExecuteGameplayCueLocal` _asc (struct :`TagName` "GameplayCue.Weapon.GrenadeLauncher.Impact") (`AbilitySystemBlueprintLibrary.MakeGameplayCueParameters` 0.0 0.0 (struct) (struct) (struct) (struct) (struct) (`self.K2_GetActorLocation`)))
      (bind _asbp_survivor (cast `/Game/Survival/Blueprints/Characters/BP_Survivor` (`self.GetInstigator`)))
      (bind _asplayer_controller (cast `PlayerController` (`Pawn.GetController` _asbp_survivor)))
      (bind _returnvalue (`KismetMathLibrary.Vector_Distance` (`self.K2_GetActorLocation` _asbp_survivor) (`self.K2_GetActorLocation`)))
      (if (<= _returnvalue (`self.MaxDist`))
        (`PlayerController.ClientStartCameraShake` :`self` _asplayer_controller :`Shake` "/Game/Survival/Blueprints/CameraShake/BP_GrenadeImpactCamShake.BP_GrenadeImpactCamShake_C" :`Scale` (`KismetMathLibrary.FClamp` (/ (`self.MaxDist`) _returnvalue)))))
    (:`else`)))

(fn `UserConstructionScript`)