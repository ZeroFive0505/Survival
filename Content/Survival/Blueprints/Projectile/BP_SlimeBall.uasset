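; BP_SlimeBall is a slime projectile that damages survivors it hits and destroys itself on impact.
; On sphere hit against a BP_Survivor, it adds the survivor as a target to a preset damage effect container spec and applies it through the Gameplay Ability System.
; It then calls HitBy with its owner, provided the instigator's ability system component casts to GSAbilitySystemComponent.
; Hits on anything else simply destroy the ball.
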(event `self.Sphere.OnComponentHit`
  (params (HitComponent :type "PrimitiveComponent Object Reference") (OtherActor :type "Actor Object Reference") (OtherComp :type "PrimitiveComponent Object Reference") (NormalImpulse :type "Vector Structure") (Hit :type "HitResult Structure (by ref)"))
  (bind _asbp_survivor (cast `/Game/Survival/Blueprints/Characters/BP_Survivor` OtherActor)
    (:`then`
      (`GSBlueprintFunctionLibrary.AddTargetsToEffectContainerSpec` :`ContainerSpec` (`self.DamageEffectContainerSpec`) :`TargetActors` (`|MakeArray` _asbp_survivor :!type "Actor Object Reference"))
      (`GSBlueprintFunctionLibrary.ApplyExternalEffectContainerSpec` (`self.DamageEffectContainerSpec`))
      (cast `GSAbilitySystemComponent` (`AbilitySystemBlueprintLibrary.GetAbilitySystemComponent` (`self.Instigator`)))
      (`GSSurvivor.HitBy` _asbp_survivor (`self.GetOwner`)))
    (:`CastFailed`
      _))
  (`self.K2_DestroyActor`))

(fn `UserConstructionScript`)