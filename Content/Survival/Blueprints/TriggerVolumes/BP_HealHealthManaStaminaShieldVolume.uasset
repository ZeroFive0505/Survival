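; Trigger volume that periodically applies a gameplay effect to a living GSCharacter inside it, named for restoring health, mana, stamina and shield.
; Box overlap starts a server-side looping timer using HealPerSec as its interval, applying EffectClass through the character's Ability System Component.
; It tracks one timer handle and the latest overlapping actor, so any end overlap clears only the most recent timer.
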(event `self.Box.OnComponentBeginOverlap`
  (params (OverlappedComponent :type "PrimitiveComponent Object Reference") (OtherActor :type "Actor Object Reference") (OtherComp :type "PrimitiveComponent Object Reference") (OtherBodyIndex :type Integer) (bFromSweep :type Boolean) (SweepResult :type "HitResult Structure (by ref)"))
  (`/Engine/EditorBlueprintResources/ActorMacros.Switch Has Authority`
    (:`Authority`
      (bind _returnvalue (`KismetSystemLibrary.K2_SetTimerDelegate` (delegate `HealTick`) (`self.HealPerSec`) true)))))

(event `HealTick`
  (`/Engine/EditorBlueprintResources/ActorMacros.Switch Has Authority`
    (:`Authority`
      (bind _asgscharacter (cast `GSCharacter` (stale `self.Box.OnComponentBeginOverlap` OtherActor)))
      (bind _returnvalue (`AbilitySystemBlueprintLibrary.GetAbilitySystemComponent` _asgscharacter))
      (if (and (`GSCharacter.IsAlive` _asgscharacter) (`KismetSystemLibrary.IsValid` _returnvalue))
        (`AbilitySystemComponent.BP_ApplyGameplayEffectToSelf` _returnvalue (`self.EffectClass`) 1.0 (`AbilitySystemComponent.MakeEffectContext` _returnvalue))))))

(event `self.Box.OnComponentEndOverlap`
  (params (OverlappedComponent :type "PrimitiveComponent Object Reference") (OtherActor :type "Actor Object Reference") (OtherComp :type "PrimitiveComponent Object Reference") (OtherBodyIndex :type Integer))
  (if (`KismetSystemLibrary.K2_IsValidTimerHandle` (stale `self.Box.OnComponentBeginOverlap` _returnvalue))
    (`KismetSystemLibrary.K2_ClearAndInvalidateTimerHandle` (stale `self.Box.OnComponentBeginOverlap` _returnvalue))))

(fn `UserConstructionScript`)