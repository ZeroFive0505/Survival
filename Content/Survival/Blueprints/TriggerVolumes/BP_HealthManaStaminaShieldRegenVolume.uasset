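; Trigger volume that, judging by its name, grants health, mana, stamina and shield regeneration through the Gameplay Ability System.
; When a living GSCharacter enters the box, it applies the configured EffectClass gameplay effect to that character's ability system component at level 1.
; On exit it removes all stacks of that effect class, provided the character is still alive.
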(event `self.Box.OnComponentBeginOverlap`
  (params (OverlappedComponent :type "PrimitiveComponent Object Reference") (OtherActor :type "Actor Object Reference") (OtherComp :type "PrimitiveComponent Object Reference") (OtherBodyIndex :type Integer) (bFromSweep :type Boolean) (SweepResult :type "HitResult Structure (by ref)"))
  (bind _asgscharacter (cast `GSCharacter` OtherActor))
  (bind _returnvalue (`AbilitySystemBlueprintLibrary.GetAbilitySystemComponent` _asgscharacter))
  (if (and (`GSCharacter.IsAlive` _asgscharacter) (`KismetSystemLibrary.IsValid` _returnvalue))
    (bind _effectclass (`self.EffectClass`)
      (:`then`
        (`AbilitySystemComponent.BP_ApplyGameplayEffectToSelf` _returnvalue _effectclass 1.0 (`AbilitySystemComponent.MakeEffectContext` _returnvalue)))
      (:`else`))))

(event `self.Box.OnComponentEndOverlap`
  (params (OverlappedComponent :type "PrimitiveComponent Object Reference") (OtherActor :type "Actor Object Reference") (OtherComp :type "PrimitiveComponent Object Reference") (OtherBodyIndex :type Integer))
  (bind _asgscharacter (cast `GSCharacter` OtherActor))
  (bind _returnvalue (`AbilitySystemBlueprintLibrary.GetAbilitySystemComponent` _asgscharacter))
  (if (and (`GSCharacter.IsAlive` _asgscharacter) (`KismetSystemLibrary.IsValid` _returnvalue))
    (bind _effectclass (`self.EffectClass`)
      (:`then`
        (`AbilitySystemComponent.RemoveActiveGameplayEffectBySourceEffect` _returnvalue _effectclass null -1))
      (:`else`))))

(fn `UserConstructionScript`)