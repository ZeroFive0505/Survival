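; BP_DamageVolume is a trigger volume that deals periodic damage to characters inside its box through the Gameplay Ability System.
; On the server, begin overlap starts a looping timer at DamagePerSec intervals, applying EffectClass to a living GSCharacter with Damage as the Data.Damage SetByCaller magnitude.
; It stores one timer handle and reads the actor from the latest begin overlap, and any end overlap clears that timer.
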(event `self.Box.OnComponentBeginOverlap`
  (params (OverlappedComponent :type "PrimitiveComponent Object Reference") (OtherActor :type "Actor Object Reference") (OtherComp :type "PrimitiveComponent Object Reference") (OtherBodyIndex :type Integer) (bFromSweep :type Boolean) (SweepResult :type "HitResult Structure (by ref)"))
  (`/Engine/EditorBlueprintResources/ActorMacros.Switch Has Authority`
    (:`Authority`
      (bind _returnvalue (`KismetSystemLibrary.K2_SetTimerDelegate` (delegate `DamageTick`) (`self.DamagePerSec`) true)))))

(event `DamageTick`
  (`/Engine/EditorBlueprintResources/ActorMacros.Switch Has Authority`
    (:`Authority`
      (bind _asgscharacter (cast `GSCharacter` (stale `self.Box.OnComponentBeginOverlap` OtherActor)))
      (bind _returnvalue (`AbilitySystemBlueprintLibrary.GetAbilitySystemComponent` _asgscharacter))
      (if (and (`GSCharacter.IsAlive` _asgscharacter) (`KismetSystemLibrary.IsValid` _returnvalue))
        (bind _returnvalue_2 (`AbilitySystemBlueprintLibrary.AssignTagSetByCallerMagnitude` (`AbilitySystemComponent.MakeOutgoingSpec` _returnvalue (`self.EffectClass`) 1.0 (`AbilitySystemComponent.MakeEffectContext` _returnvalue)) (struct :`TagName` "Data.Damage") (`self.Damage`)))
        (`AbilitySystemComponent.BP_ApplyGameplayEffectSpecToSelf` _returnvalue _returnvalue_2)))))

(event `self.Box.OnComponentEndOverlap`
  (params (OverlappedComponent :type "PrimitiveComponent Object Reference") (OtherActor :type "Actor Object Reference") (OtherComp :type "PrimitiveComponent Object Reference") (OtherBodyIndex :type Integer))
  (if (`KismetSystemLibrary.K2_IsValidTimerHandle` (stale `self.Box.OnComponentBeginOverlap` _returnvalue))
    (`KismetSystemLibrary.K2_ClearAndInvalidateTimerHandle` (stale `self.Box.OnComponentBeginOverlap` _returnvalue))))

(fn `UserConstructionScript`)