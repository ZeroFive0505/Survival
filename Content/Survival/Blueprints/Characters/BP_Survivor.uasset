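; BP_Survivor is the player survivor character for the Survival game.
; On begin play it adds a damage indicator widget and registers for the game mode's wave-finish event.
; Each finished wave grants gold through a Gameplay Ability System effect with a SetByCaller magnitude.
; Hits shake the camera and update the indicator; death spawns a death pawn as view target, hides the survivor and plays a sound.
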(event `self.ReceiveBeginPlay`
  (bind _asplayer_controller (cast `PlayerController` (`self.GetController`)))
  (bind _returnvalue (`|CreateWidget` "/Game/Survival/Blueprints/UI/WBP_DamageIndicator.WBP_DamageIndicator_C" _asplayer_controller self))
  (bind _output_get (set `self.Indicator` _returnvalue))
  (`UserWidget.AddToViewport` _output_get 20)
  (bind _asbp_game_mode (cast `/Game/Survival/Blueprints/GameMode/BP_GameMode` (`GameplayStatics.GetGameMode`)))
  (add `/Game/Survival/Blueprints/GameMode/BP_GameMode.WaveFinish` _asbp_game_mode (delegate `OnWaveFinish`)))

(event `OnWaveFinish`
  (bind _returnvalue (`AbilitySystemBlueprintLibrary.GetAbilitySystemComponent` self))
  (bind _returnvalue_2 (`AbilitySystemBlueprintLibrary.AssignTagSetByCallerMagnitude` (`AbilitySystemComponent.MakeOutgoingSpec` _returnvalue "/Game/Survival/Blueprints/GameplayEffects/Items/GE_GoldAdd.GE_GoldAdd_C" 1.0 (`AbilitySystemComponent.MakeEffectContext` _returnvalue)) (struct :`TagName` "Data.Gold") 500.0))
  (`AbilitySystemComponent.BP_ApplyGameplayEffectSpecToSelf` _returnvalue _returnvalue_2))

(event `self.ReceiveTick`
  (params (DeltaSeconds :type "Float (single-precision)")))

(event `self.SpawnDeathPawn`
  (bind _returnvalue (`|SpawnActorFromClass` "/Game/Survival/Blueprints/Characters/BP_DeathPawn.BP_DeathPawn_C" (`self.GetTransform`) "AlwaysSpawn" "MultiplyWithRoot" null null))
  (`PlayerController.SetViewTargetWithBlend` (`GameplayStatics.GetPlayerController` 0) _returnvalue 0.0 "VTBlend_Linear" 0.0 false)
  (`self.SetActorHiddenInGame` true)
  (`GameplayStatics.PlaySound2D` (`self.DeathSound`) 1.0 1.0 0.0 null null))

(event `self.HitBy`
  (params (DamageCauser :type "Actor Object Reference"))
  (`PlayerController.ClientStartCameraShake` :`self` (`GameplayStatics.GetPlayerController` 0) :`Shake` "/Game/Survival/Blueprints/CameraShake/BP_HitCamShake.BP_HitCamShake_C" :`PlaySpace` "World")
  (`/Game/Survival/Blueprints/UI/WBP_DamageIndicator.Hit` (`self.Indicator`) DamageCauser))

(fn `UserConstructionScript`)