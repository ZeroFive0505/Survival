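; BP_DeathPawn is a death pawn built around a Cube that gets thrown into a random tumble when spawned.
; On BeginPlay it applies a scaled random impulse to the Cube at a random, equally scaled location, adding spin as well as movement.
; A coin flip then fires either the left or the right radial force component for an extra shove.
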(event `self.ReceiveBeginPlay`
  (bind _returnvalue (`KismetMathLibrary.RandomFloatInRange` -10.0 10.0))
  (bind _returnvalue_2 (* (`KismetMathLibrary.MakeVector` _returnvalue _returnvalue _returnvalue) 600.0))
  (`PrimitiveComponent.AddImpulseAtLocation` (`self.Cube`) _returnvalue_2 _returnvalue_2 "None")
  (if (`KismetMathLibrary.RandomBool`)
    (`RadialForceComponent.FireImpulse` (`self.LeftRadialForce`))
    (else
      (`RadialForceComponent.FireImpulse` (`self.RIghtRadialForce`)))))

(fn `UserConstructionScript`)