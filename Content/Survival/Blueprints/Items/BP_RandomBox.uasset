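; Purchasable loot chest that players open by interacting with its lock, spawning random weapons nearby.
; On the server, interaction checks the survivor's funds, then applies the open effect and deducts the price via GAS, or shows a not-enough-money notice.
; A gameplay tag listener drives lid rotation and lock animation for opening and closing.
; Opening also fires a gameplay cue and runs an EQS query for spawn points, skipping those blocked by a sphere trace.
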(event `SpawnAtRandomLocation`
  (bind _returnvalue (`EnvQueryManager.RunEQSQuery` "/Game/Survival/Blueprints/Items/EQS_SpawnLocation.EQS_SpawnLocation" self "AllMatching"))
  (add `EnvQueryInstanceBlueprintWrapper.OnQueryFinishedEvent` _returnvalue (delegate `OnQueryEnd`)))

(event `self.ReceiveBeginPlay`
  (`MovementComponent.SetUpdatedComponent` (`self.RotatingMovement`) (`self.Top`))
  (bind (_asynctaskproxy _tag) (`AsyncTaskGameplayTagAddedRemoved.ListenForGameplayTagAddedOrRemoved` (`AbilitySystemBlueprintLibrary.GetAbilitySystemComponent` self) (`self.ListenTags`))
    (:`then`
      (set `self.ListenForTagAddRemotedTask` _asynctaskproxy)
      (set `self.LockStartingRelativeLocation` (`SceneComponent.RelativeLocation` (`self.Lock`))))
    (:`OnTagAdded`
      (bind _returnvalue (== _tag (`self.OpenTag`)))
      (if _returnvalue
        (`self.OpenRandomBox`)))
    (:`OnTagRemoved`
      (if _returnvalue
        (`self.CloseRandomBox`)))))

(event `OnQueryEnd`
  (params (QueryInstance :type "EnvQueryInstanceBlueprintWrapper Object Reference") (QueryStatus :type "EEnvQueryStatus Enum" :default "Processing"))
  (bind _weapon (`self.Weapon`))
  (bind _resultlocations (`EnvQueryInstanceBlueprintWrapper.GetQueryResultsAsLocations` QueryInstance))
  (`KismetArrayLibrary.Array_Shuffle` (`self.Weapon`))
  (`KismetArrayLibrary.Array_Shuffle` _resultlocations)
  (for _index (range (+ (+ (`KismetMathLibrary.RandomInteger` 5) 1) 1))
    (bind _output (`|GetArrayItem` _resultlocations _index))
    (bind (_outhit _returnvalue) (`KismetSystemLibrary.SphereTraceSingleForObjects` _output _output 32.0 (`|MakeArray` "ObjectTypeQuery12" :!type "EObjectTypeQuery Enum")))
    (if (not _returnvalue)
      (`|SpawnActorFromClass` (`|GetArrayItem` _weapon (`KismetMathLibrary.RandomInteger` (`KismetArrayLibrary.Array_Length` _weapon))) (`KismetMathLibrary.MakeTransform` (+ _output (0.0 0.0 50.0))) "Undefined" "MultiplyWithRoot" null null))))

(event `self.PreInteract`
  (params (InteractingActor :type "Actor Object Reference") (InteractionComponent :type "PrimitiveComponent Object Reference"))
  (bind _returnvalue (`AbilitySystemBlueprintLibrary.GetAbilitySystemComponent` self))
  (if (== InteractionComponent (`self.Lock`))
    (`/Engine/EditorBlueprintResources/ActorMacros.Switch Has Authority`
      (:`Authority`
        (bind _returnvalue_2 (`AbilitySystemComponent.BP_ApplyGameplayEffectToSelf` _returnvalue "/Game/Survival/Blueprints/GameplayEffects/Survivor/GE_Interacting.GE_Interacting_C" 0.0 (`AbilitySystemComponent.MakeEffectContext` _returnvalue)))
        (set `self.GE_InteractingHandle` _returnvalue_2)))))

(event `self.PostInteract`
  (params (InteractingActor :type "Actor Object Reference") (InteractionComponent :type "PrimitiveComponent Object Reference"))
  (bind _returnvalue (`AbilitySystemBlueprintLibrary.GetAbilitySystemComponent` InteractingActor))
  (bind _abilitysystem (`self.AbilitySystem`))
  (if (== InteractionComponent (`self.Lock`))
    (`/Engine/EditorBlueprintResources/ActorMacros.Switch Has Authority`
      (:`Authority`
        (bind _asbp_survivor (cast `/Game/Survival/Blueprints/Characters/BP_Survivor` InteractingActor))
        (bind _asplayer_controller (cast `PlayerController` (`Pawn.GetController` _asbp_survivor)))
        (if (>= (`.ReturnValue` (`AbilitySystemBlueprintLibrary.GetFloatAttributeFromAbilitySystemComponent` _returnvalue (struct :`AttributeName` "Gold" :`Attribute` "/Script/GASSurvival.GSAttributeSetBase:Gold" :`AttributeOwner` "/Script/CoreUObject.Class'\"/Script/GASSurvival.GSAttributeSetBase\"'"))) (`self.Price`))
          (`AbilitySystemComponent.BP_ApplyGameplayEffectToTarget` _returnvalue "/Game/Survival/Blueprints/GameplayEffects/Items/GE_RandomBoxOpen.GE_RandomBoxOpen_C" (`AbilitySystemBlueprintLibrary.GetAbilitySystemComponent` self) 0.0 (`AbilitySystemComponent.MakeEffectContext` _returnvalue))
          (`AbilitySystemComponent.RemoveActiveGameplayEffect` (`AbilitySystemBlueprintLibrary.GetAbilitySystemComponent` self) (`self.GE_InteractingHandle`) -1)
          (bind _returnvalue_2 (`AbilitySystemBlueprintLibrary.AssignTagSetByCallerMagnitude` (`AbilitySystemComponent.MakeOutgoingSpec` _abilitysystem "/Game/Survival/Blueprints/GameplayEffects/Items/GE_GoldAdd.GE_GoldAdd_C" 1.0 (`AbilitySystemComponent.MakeEffectContext` _abilitysystem)) (struct :`TagName` "Data.Gold") (`KismetMathLibrary.Conv_IntToDouble` (* (`self.Price`) -1))))
          (`AbilitySystemComponent.BP_ApplyGameplayEffectSpecToTarget` (`self.AbilitySystem`) _returnvalue_2 _returnvalue)
          (else
            (bind _returnvalue_3 (`|CreateWidget` "/Game/Survival/Blueprints/UI/WBP_UserNoticeMessage.WBP_UserNoticeMessage_C" _asplayer_controller "You do not have enough money!"))
            (`UserWidget.AddToViewport` _returnvalue_3 20)
            (`KismetSystemLibrary.Delay` 2.0)
            (`Widget.RemoveFromParent` _returnvalue_3)))))))

(event `OpenRandomBox`
  (bind (_lockstartingrelativelocation_x _lockstartingrelativelocation_y _lockstartingrelativelocation_z) (`KismetMathLibrary.BreakVector` (`self.LockStartingRelativeLocation`)))
  (set `RotatingMovementComponent.RotationRate` (struct :`Pitch` 180.0) (`self.RotatingMovement`))
  (`ActorComponent.Activate` (`self.RotatingMovement`) true)
  (`|ExecutionSequence`
    (:`then_0`
      (`KismetSystemLibrary.Delay` (`self.ChestTopAnimationDuration`))
      (`MovementComponent.StopMovementImmediately` (`self.RotatingMovement`))
      (`ActorComponent.Deactivate` (`self.RotatingMovement`))
      (`self.SpawnAtRandomLocation`)
      (`GameplayCueFunctionLibrary.ExecuteGameplayCueOnActor` self (struct :`TagName` "GameplayCue.Chest.Open") (`AbilitySystemBlueprintLibrary.MakeGameplayCueParameters` 0.0 0.0 (`AbilitySystemComponent.MakeEffectContext` (`self.AbilitySystem`)) (struct) (struct) (struct) (struct) (`self.K2_GetActorLocation` self) (0.0 0.0 0.0) self null self)))
    (:`then_1`
      (bind (_direction _time) (`Timeline|LockFallOff`)
        (:`Update`
          (`SceneComponent.K2_SetRelativeLocation` (`self.Lock`) (`KismetMathLibrary.MakeVector` _lockstartingrelativelocation_x _lockstartingrelativelocation_y (`KismetMathLibrary.Lerp` _lockstartingrelativelocation_z (- _lockstartingrelativelocation_z 60.0) (/ _time 0.2))) false false))
        (:`Finished`
          (`SceneComponent.SetVisibility` (`self.Lock`) false true))))))

(event `CloseRandomBox`
  (set `RotatingMovementComponent.RotationRate` (struct :`Pitch` -180.0) (`self.RotatingMovement`))
  (`ActorComponent.Activate` (`self.RotatingMovement`) true)
  (`KismetSystemLibrary.Delay` (`self.ChestTopAnimationDuration`))
  (`MovementComponent.StopMovementImmediately` (`self.RotatingMovement`))
  (`ActorComponent.Deactivate` (`self.RotatingMovement`))
  (`SceneComponent.SetVisibility` (`self.Lock`) true true)
  (`SceneComponent.K2_SetRelativeLocation` (`self.Lock`) (`self.LockStartingRelativeLocation`) false false))

(event `self.CancelInteraction`
  (params (InteractionComponent :type "PrimitiveComponent Object Reference"))
  (if (== InteractionComponent (`self.Lock`))
    (`AbilitySystemComponent.RemoveActiveGameplayEffect` (`AbilitySystemBlueprintLibrary.GetAbilitySystemComponent` self) (`self.GE_InteractingHandle`) -1)))

(event `self.ReceiveEndPlay`
  (params (EndPlayReason :type "EEndPlayReason Enum" :default "Destroyed"))
  (bind _listenfortagaddremotedtask (`self.ListenForTagAddRemotedTask`)
    (:`then`
      (`AsyncTaskGameplayTagAddedRemoved.EndTask` _listenfortagaddremotedtask))
    (:`else`)))

(fn `GetInteractionDescription`
  (params (InteractionComponent :type "PrimitiveComponent Object Reference"))
  (returns (ReturnValue :type Text))
  (return (`|FormatText` "Open Random Box {Price}$" (`self.Price`))))

(fn `GetInteractionDuration`
  (params (InteractionComponent :type "PrimitiveComponent Object Reference"))
  (returns (ReturnValue :type "Float (single-precision)"))
  (if (== InteractionComponent (`self.Lock`))
    (return (`self.OpenInteractionDuration`))
    (else
      (return -1.0))))

(fn `GetPostInteractSyncType`
  (params (InteractionComponent :type "PrimitiveComponent Object Reference"))
  (returns (bShouldSync :type Boolean) (Type :type "EAbilityTaskNetSyncType Enum"))
  (if (== InteractionComponent (`self.Lock`))
    (return false "OnlyServerWait")
    (else
      (return false "OnlyServerWait"))))

(fn `GetPreInteractSyncType`
  (params (InteractionComponent :type "PrimitiveComponent Object Reference"))
  (returns (bShouldSync :type Boolean) (Type :type "EAbilityTaskNetSyncType Enum"))
  (if (== InteractionComponent (`self.Lock`))
    (return true "OnlyClientWait")
    (else
      (return false "BothWait"))))

(fn `IsAvailableForInteraction`
  (params (InteractionComponent :type "PrimitiveComponent Object Reference"))
  (returns (ReturnValue :type Boolean))
  (return (and (== InteractionComponent (`self.Lock`)) (not (`GameplayTagAssetInterface.HasAnyMatchingGameplayTags` (`AbilitySystemBlueprintLibrary.GetAbilitySystemComponent` self) (`self.AvailabilityTags`))))))

(fn `UserConstructionScript`)