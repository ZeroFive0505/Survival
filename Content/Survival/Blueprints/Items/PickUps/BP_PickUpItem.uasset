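; BP_PickUpItem is a pickup actor that grants a Gameplay Ability System effect on touch and expires after a fixed lifespan set at BeginPlay.
; On sphere overlap, it has the other actor's Ability System Component apply EffectToApply to itself and fires a local GameplayCue at the pickup's location.
; The pickup destroys itself on any overlap, even when the other actor has no Ability System Component.
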(event `self.ReceiveBeginPlay`
  (`self.SetLifeSpan` 60.0))

(event `self.Sphere.OnComponentBeginOverlap`
  (params (OverlappedComponent :type "PrimitiveComponent Object Reference") (OtherActor :type "Actor Object Reference") (OtherComp :type "PrimitiveComponent Object Reference") (OtherBodyIndex :type Integer) (bFromSweep :type Boolean) (SweepResult :type "HitResult Structure (by ref)"))
  (bind _returnvalue (`AbilitySystemBlueprintLibrary.GetAbilitySystemComponent` OtherActor))
  (`/Engine/EditorBlueprintResources/StandardMacros.IsValid` _returnvalue
    (:`Is Valid`
      (`AbilitySystemComponent.BP_ApplyGameplayEffectToTarget` _returnvalue (`self.EffectToApply`) _returnvalue 0.0 (`AbilitySystemComponent.MakeEffectContext` (`self.GSAbilitySystem`)))
      (`GSAbilitySystemComponent.ExecuteGameplayCueLocal` (`self.GSAbilitySystem`) (`self.GameplayCueTag`) (`AbilitySystemBlueprintLibrary.MakeGameplayCueParameters` 0.0 0.0 (struct) (struct) (struct) (struct) (struct) (`self.K2_GetActorLocation` self) (0.0 0.0 0.0) self null self)))
    (:`Is Not Valid`
      _))
  (`self.K2_DestroyActor`))

(fn `UserConstructionScript`)