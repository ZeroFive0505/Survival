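; Gold pickup actor that grants a random amount of gold to any overlapping actor with an Ability System Component.
; On sphere overlap, its own GSAbilitySystem builds a GE_GoldAdd spec, sets the rolled amount through the Data.Gold SetByCaller tag, and applies it to that actor.
; It then executes the gold pickup GameplayCue locally at its location; this graph does not destroy the pickup.
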(event `self.Sphere.OnComponentBeginOverlap`
  (params (OverlappedComponent :type "PrimitiveComponent Object Reference") (OtherActor :type "Actor Object Reference") (OtherComp :type "PrimitiveComponent Object Reference") (OtherBodyIndex :type Integer) (bFromSweep :type Boolean) (SweepResult :type "HitResult Structure (by ref)"))
  (bind _returnvalue (`AbilitySystemBlueprintLibrary.GetAbilitySystemComponent` OtherActor))
  (bind _gsabilitysystem (`self.GSAbilitySystem`))
  (`/Engine/EditorBlueprintResources/StandardMacros.IsValid` _returnvalue
    (:`Is Valid`
      (bind _returnvalue_2 (`AbilitySystemBlueprintLibrary.AssignTagSetByCallerMagnitude` (`AbilitySystemComponent.MakeOutgoingSpec` _gsabilitysystem "/Game/Survival/Blueprints/GameplayEffects/Items/GE_GoldAdd.GE_GoldAdd_C" 1.0 (`AbilitySystemComponent.MakeEffectContext` _gsabilitysystem)) (struct :`TagName` "Data.Gold") (`KismetMathLibrary.Conv_IntToDouble` (`KismetMathLibrary.RandomIntegerInRange` 50 201))))
      (`AbilitySystemComponent.BP_ApplyGameplayEffectSpecToTarget` (`self.GSAbilitySystem`) _returnvalue_2 _returnvalue)
      (`GSAbilitySystemComponent.ExecuteGameplayCueLocal` (`self.GSAbilitySystem`) (struct :`TagName` "GameplayCue.PickUp.Gold") (`AbilitySystemBlueprintLibrary.MakeGameplayCueParameters` 0.0 0.0 (struct) (struct) (struct) (struct) (struct) (`self.K2_GetActorLocation`) (0.0 0.0 0.0) self null self)))))

(fn `UserConstructionScript`
  (`parent.UserConstructionScript`))