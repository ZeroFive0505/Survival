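; Interactable ammo shop that sells gameplay effects to survivors for gold through the Gameplay Ability System.
; Timed capsule interaction applies an interacting effect on the server, removed on completion or cancel, with availability gated by tags.
; After price and attribute-limit checks, each configured effect is applied alongside a SetByCaller gold deduction and gameplay cue.
; Failed checks show a temporary notice widget; the construction script sets the sign's title and color.
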(event `self.PreInteract`
  (params (InteractingActor :type "Actor Object Reference") (InteractionComponent :type "PrimitiveComponent Object Reference"))
  (bind _returnvalue (`AbilitySystemBlueprintLibrary.GetAbilitySystemComponent` self))
  (if (== InteractionComponent (`self.Capsule`))
    (`/Engine/EditorBlueprintResources/ActorMacros.Switch Has Authority`
      (:`Authority`
        (bind _returnvalue_2 (`AbilitySystemComponent.BP_ApplyGameplayEffectToSelf` _returnvalue "/Game/Survival/Blueprints/GameplayEffects/Survivor/GE_Interacting.GE_Interacting_C" 0.0 (`AbilitySystemComponent.MakeEffectContext` _returnvalue)))
        (set `self.GE_InteractingHandle` _returnvalue_2)))))

(event `self.PostInteract`
  (params (InteractingActor :type "Actor Object Reference") (InteractionComponent :type "PrimitiveComponent Object Reference"))
  (bind _returnvalue (`AbilitySystemBlueprintLibrary.GetAbilitySystemComponent` InteractingActor))
  (bind _abilitysystem (`self.AbilitySystem`))
  (bind _returnvalue_2 (`AbilitySystemBlueprintLibrary.GetAbilitySystemComponent` self))
  (if (== InteractionComponent (`self.Capsule`))
    (`/Engine/EditorBlueprintResources/ActorMacros.Switch Has Authority`
      (:`Authority`
        (`AbilitySystemComponent.RemoveActiveGameplayEffect` (`AbilitySystemBlueprintLibrary.GetAbilitySystemComponent` self) (`self.GE_InteractingHandle`) -1)
        (bind _asbp_survivor (cast `/Game/Survival/Blueprints/Characters/BP_Survivor` InteractingActor))
        (bind _asplayer_controller (cast `PlayerController` (`Pawn.GetController` _asbp_survivor)))
        (if (>= (`.ReturnValue` (`AbilitySystemBlueprintLibrary.GetFloatAttributeFromAbilitySystemComponent` _returnvalue (struct :`AttributeName` "Gold" :`Attribute` "/Script/GASSurvival.GSAttributeSetBase:Gold" :`AttributeOwner` "/Script/CoreUObject.Class'\"/Script/GASSurvival.GSAttributeSetBase\"'"))) (`self.Price`))
          (if (< (`.ReturnValue` (`AbilitySystemBlueprintLibrary.GetFloatAttributeFromAbilitySystemComponent` _returnvalue (struct :`AttributeName` "RifleReserveAmmo" :`Attribute` "/Script/GASSurvival.GSAmmoAttributeSet:RifleReserveAmmo" :`AttributeOwner` "/Script/CoreUObject.Class'\"/Script/GASSurvival.GSAmmoAttributeSet\"'"))) (`.ReturnValue` (`AbilitySystemBlueprintLibrary.GetFloatAttributeFromAbilitySystemComponent` _returnvalue (struct :`AttributeName` "MaxRifleReserveAmmo" :`Attribute` "/Script/GASSurvival.GSAmmoAttributeSet:MaxRifleReserveAmmo" :`AttributeOwner` "/Script/CoreUObject.Class'\"/Script/GASSurvival.GSAmmoAttributeSet\"'"))))
            (for _array_element (`self.EffectClasses`)
              (`AbilitySystemComponent.BP_ApplyGameplayEffectSpecToSelf` _returnvalue (`AbilitySystemComponent.MakeOutgoingSpec` _returnvalue_2 _array_element 1.0 (`AbilitySystemComponent.MakeEffectContext` _returnvalue_2)))
              (bind _returnvalue_3 (`AbilitySystemBlueprintLibrary.AssignTagSetByCallerMagnitude` (`AbilitySystemComponent.MakeOutgoingSpec` _abilitysystem "/Game/Survival/Blueprints/GameplayEffects/Items/GE_GoldAdd.GE_GoldAdd_C" 1.0 (`AbilitySystemComponent.MakeEffectContext` _abilitysystem)) (struct :`TagName` "Data.Gold") (`KismetMathLibrary.Conv_IntToDouble` (* (`self.Price`) -1))))
              (`AbilitySystemComponent.BP_ApplyGameplayEffectSpecToTarget` _abilitysystem _returnvalue_3 _returnvalue)
              (`GameplayCueFunctionLibrary.ExecuteGameplayCueOnActor` self (`self.GameplayCueTag`) (`AbilitySystemBlueprintLibrary.MakeGameplayCueParameters` 0.0 0.0 (struct) (struct) (struct) (struct) (struct) (`self.K2_GetActorLocation`) (0.0 0.0 0.0) self null self)))
            (else
              (bind _returnvalue_4 (`|CreateWidget` "/Game/Survival/Blueprints/UI/WBP_UserNoticeMessage.WBP_UserNoticeMessage_C" _asplayer_controller ""))
              (`UserWidget.AddToViewport` _returnvalue_4 20)
              (`KismetSystemLibrary.Delay` 2.0)
              (`Widget.RemoveFromParent` _returnvalue_4)))
          (else
            (bind _returnvalue_5 (`|CreateWidget` "/Game/Survival/Blueprints/UI/WBP_UserNoticeMessage.WBP_UserNoticeMessage_C" _asplayer_controller "You do not have enough money!"))
            (`UserWidget.AddToViewport` _returnvalue_5 20)
            (`KismetSystemLibrary.Delay` 2.0)
            (`Widget.RemoveFromParent` _returnvalue_5)))))))

(event `self.ReceiveEndPlay`
  (params (EndPlayReason :type "EEndPlayReason Enum" :default "Destroyed"))
  (bind _listenfortagaddremovedtask (`self.ListenForTagAddRemovedTask`)
    (:`then`
      (`AsyncTaskGameplayTagAddedRemoved.EndTask` _listenfortagaddremovedtask))
    (:`else`)))

(event `self.CancelInteraction`
  (params (InteractionComponent :type "PrimitiveComponent Object Reference"))
  (if (== InteractionComponent (`self.Capsule`))
    (`AbilitySystemComponent.RemoveActiveGameplayEffect` (`AbilitySystemBlueprintLibrary.GetAbilitySystemComponent` self) (`self.GE_InteractingHandle`) -1)))

(fn `GetInteractionDescription`
  (params (InteractionComponent :type "PrimitiveComponent Object Reference"))
  (returns (ReturnValue :type Text))
  (return "Description"))

(fn `GetInteractionDuration`
  (params (InteractionComponent :type "PrimitiveComponent Object Reference"))
  (returns (ReturnValue :type "Float (single-precision)"))
  (if (== InteractionComponent (`self.Capsule`))
    (return (`self.PurchaseInteractionDuration`))
    (else
      (return -1.0))))

(fn `GetPostInteractSyncType`
  (params (InteractionComponent :type "PrimitiveComponent Object Reference"))
  (returns (bShouldSync :type Boolean) (Type :type "EAbilityTaskNetSyncType Enum"))
  (if (== InteractionComponent (`self.Capsule`))
    (return false "OnlyServerWait")
    (else
      (return false "BothWait"))))

(fn `GetPreInteractSyncType`
  (params (InteractionComponent :type "PrimitiveComponent Object Reference"))
  (returns (bShouldSync :type Boolean) (Type :type "EAbilityTaskNetSyncType Enum"))
  (if (== InteractionComponent (`self.Capsule`))
    (return true "OnlyClientWait")
    (else
      (return false "BothWait"))))

(fn `IsAvailableForInteraction`
  (params (InteractionComponent :type "PrimitiveComponent Object Reference"))
  (returns (ReturnValue :type Boolean))
  (return (and (== InteractionComponent (`self.Capsule`)) (not (`GameplayTagAssetInterface.HasAnyMatchingGameplayTags` (`AbilitySystemBlueprintLibrary.GetAbilitySystemComponent` self) (`self.AvailabilityTags`))))))

(fn `UserConstructionScript`
  (`TextRenderComponent.K2_SetText` (`self.TextRender`) (`self.ShopTitle`))
  (`TextRenderComponent.SetTextRenderColor` (`self.TextRender`) (`KismetMathLibrary.Conv_LinearColorToColor` (`self.Color`))))