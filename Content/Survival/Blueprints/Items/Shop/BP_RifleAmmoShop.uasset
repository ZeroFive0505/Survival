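; BP_RifleAmmoShop is an interactable shop item for buying rifle ammo in the Survival game.
; It overrides the interaction description to show a buy prompt formatted with its Price variable.
; All other interaction events and queries, including availability, duration and sync types, pass straight to the parent Blueprint, and no purchase logic appears in this graph.
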(event `self.PreInteract`
  (params (InteractingActor :type "Actor Object Reference") (InteractionComponent :type "PrimitiveComponent Object Reference"))
  (`parent.PreInteract` InteractingActor InteractionComponent))

(event `self.PostInteract`
  (params (InteractingActor :type "Actor Object Reference") (InteractionComponent :type "PrimitiveComponent Object Reference"))
  (`parent.PostInteract` InteractingActor InteractionComponent))

(event `self.CancelInteraction`
  (params (InteractionComponent :type "PrimitiveComponent Object Reference"))
  (`parent.CancelInteraction` InteractionComponent))

(fn `GetInteractionDescription`
  (params (InteractionComponent :type "PrimitiveComponent Object Reference"))
  (returns (ReturnValue :type Text))
  (return (`|FormatText` "Buy Rifle Ammo {Price}$" (`self.Price`))))

(fn `GetInteractionDuration`
  (params (InteractionComponent :type "PrimitiveComponent Object Reference"))
  (returns (ReturnValue :type "Float (single-precision)"))
  (return (`parent.GetInteractionDuration` InteractionComponent)))

(fn `GetPostInteractSyncType`
  (params (InteractionComponent :type "PrimitiveComponent Object Reference"))
  (returns (bShouldSync :type Boolean) (Type :type "EAbilityTaskNetSyncType Enum"))
  (bind (_bshouldsync _type) (`parent.GetPostInteractSyncType` InteractionComponent))
  (return _bshouldsync _type))

(fn `GetPreInteractSyncType`
  (params (InteractionComponent :type "PrimitiveComponent Object Reference"))
  (returns (bShouldSync :type Boolean) (Type :type "EAbilityTaskNetSyncType Enum"))
  (bind (_bshouldsync _type) (`parent.GetPreInteractSyncType` InteractionComponent))
  (return _bshouldsync _type))

(fn `IsAvailableForInteraction`
  (params (InteractionComponent :type "PrimitiveComponent Object Reference"))
  (returns (ReturnValue :type Boolean))
  (return (`parent.IsAvailableForInteraction` InteractionComponent)))

(fn `UserConstructionScript`)