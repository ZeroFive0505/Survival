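; Goblin enemy weapon that equips its owning character with gameplay abilities and targeting actors.
; On BeginPlay, if the owner is valid, it grants each listed ability to the owner's Ability System Component with itself as source object, storing the spec handles.
; It then spawns reusable sphere-trace and line-trace GAS target actors.
; On destruction it destroys both trace actors but leaves the granted abilities in place.
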(event `self.ReceiveBeginPlay`
  (bind _ownercharacter (`self.OwnerCharacter`)
    (:`then`
      (for _array_element (`self.Abilities`)
        (bind _returnvalue (`GSBlueprintFunctionLibrary.GiveAbilityWithSource` (`AbilitySystemBlueprintLibrary.GetAbilitySystemComponent` _ownercharacter) _array_element 0 -1 self))
        (`KismetArrayLibrary.Array_Add` (`self.AbilitySpecHandle`) _returnvalue))
      (bind _returnvalue_2 (`|SpawnActorFromClass` "/Script/GASSurvival.GSGATA_SphereTrace" (`KismetMathLibrary.MakeTransform` (0.0 0.0 0.0)) "AlwaysSpawn" "MultiplyWithRoot" self 100.0 999999.0 (struct :`Name` "EnemyAttack") true 1 1 false false false (struct) (struct) null (struct) false null))
      (set `self.SphereTraceActor` _returnvalue_2)
      (bind _returnvalue_3 (`|SpawnActorFromClass` "/Script/GASSurvival.GSGATA_LineTrace" (`KismetMathLibrary.MakeTransform` (0.0 0.0 0.0)) "Undefined" "MultiplyWithRoot" null 999999.0 (struct :`Name` "EnemyAttack") true 1 1 false false false (struct) (struct) null (struct) false null))
      (set `self.LineTraceActor` _returnvalue_3))
    (:`else`)))

(event `self.ReceiveDestroyed`
  (`self.K2_DestroyActor` (`self.SphereTraceActor`))
  (`self.K2_DestroyActor` (`self.LineTraceActor`)))

(fn `UserConstructionScript`)