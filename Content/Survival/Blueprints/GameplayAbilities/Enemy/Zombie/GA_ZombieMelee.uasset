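; Zombie melee gameplay ability that acts as the outer wrapper for GA_ZombieMeleeInstant, modelled as a separate instant ability on the same weapon.
; On activation it lazily caches the source zombie weapon, owning zombie, instant ability's handle and instance, and the weapon's sphere trace actor.
; It then triggers the instant ability through a batched RPC activation without ending it immediately.
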(event `self.K2_ActivateAbility`
  (`self.ActivationSetUp`)
  (`self.BatchRPCTryActivateAbility` (`self.InstantAbilityHandle`)))

(event `self.K2_OnEndAbility`
  (params (bWasCancelled :type Boolean))
  (`parent.K2_OnEndAbility` bWasCancelled))

(fn `ActivationSetUp`
  (`self.SourceWeapon`
    (:`then`
      _)
    (:`else`
      (bind _asbp_zombie_weapon (cast `/Game/Survival/Blueprints/Weapon/Enemy/BP_ZombieWeapon` (`self.GetCurrentSourceObject`)))
      (set `self.SourceWeapon` _asbp_zombie_weapon)))
  (`self.OwningZombie`
    (:`then`
      _)
    (:`else`
      (bind _asbp_zombie (cast `/Game/Survival/Blueprints/Enemy/BP_Zombie` (`self.GetAvatarActorFromActorInfo`)))
      (set `self.OwningZombie` _asbp_zombie)))
  (if (not (`GSBlueprintFunctionLibrary.IsAbilitySpecHandleValid` (`self.InstantAbilityHandle`)))
    (bind _asgsability_system_component (cast `GSAbilitySystemComponent` (`self.GetAbilitySystemComponentFromActorInfo`)))
    (set `self.InstantAbilityHandle` (`GSAbilitySystemComponent.FindAbilitySpecHandleForClass` _asgsability_system_component "/Game/Survival/Blueprints/GameplayAbilities/Enemy/Zombie/GA_ZombieMeleeInstant.GA_ZombieMeleeInstant_C" (`self.SourceWeapon`))))
  (`self.InstantAbility`
    (:`then`
      _)
    (:`else`
      (bind _returnvalue (`GSBlueprintFunctionLibrary.GetPrimaryAbilityInstanceFromHandle` (`self.GetAbilitySystemComponentFromActorInfo`) (`self.InstantAbilityHandle`)))
      (bind _asga_zombie_melee_instant (cast `/Game/Survival/Blueprints/GameplayAbilities/Enemy/Zombie/GA_ZombieMeleeInstant` _returnvalue))
      (set `self.InstantAbility` _asga_zombie_melee_instant)))
  (`self.SphereTraceActor`
    (:`then`
      _)
    (:`else`
      (set `self.SphereTraceActor` (`/Game/Survival/Blueprints/Weapon/Enemy/BP_ZombieWeapon.SphereTraceActor` (`self.SourceWeapon`)))))
  (return))