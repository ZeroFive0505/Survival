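; GA_ZombieMeleeInstant is the zombie's instant melee strike ability, paired with GA_ZombieMelee, which it ends when it finishes.
; It plays the strike montage, whose Ability.Melee event triggers a net sync, a server wait for client target data and UseWeapon.
; UseWeapon fires an instant trace ahead of the zombie with the weapon's reusable SphereTraceActor and plays a local attack cue.
; Valid target data receives GE_ZombieMeleeDamage with set-by-caller damage.
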(event `self.K2_ActivateAbility`
  (`self.ActivationSetUp`)
  (`GSAT_PlayMontageForMeshAndWaitForEvent.PlayMontageForMeshAndWaitForEvent` "None" (`Character.Mesh` (`self.OwningZombie`)) "/Game/Survival/Zombie/AI/Zombie/Animations/Zombie_MeleeStrike_Montage.Zombie_MeleeStrike_Montage" (struct :`GameplayTags` (struct :`(TagName` "Ability.Melee"))) 1.0 "None" false 1.0 true 0.0 0.0
    (:`OnCompleted`
      (`AbilityTask_NetworkSyncPoint.WaitNetSync` "BothWait"
        (:`OnSync`
          (`self.K2_EndAbility`))))
    (:`OnInterrupted`
      (`self.K2_CancelAbility` :!label _label))
    (:`OnCancelled`
      (goto _label))
    (:`EventReceived`
      (`AbilityTask_NetworkSyncPoint.WaitNetSync` "OnlyServerWait"
        (:`OnSync`
          (bind (_asynctaskproxy _data) (`GSAT_ServerWaitForClientTargetData.ServerWaitForClientTargetData` "None")
            (:`then`
              (set `self.ServerWaitTargetDataTask` _asynctaskproxy)
              (`self.UseWeapon`))
            (:`ValidData`
              (`self.HandleTargetData` _data))))))))

(event `UseWeapon`
  (bind _owningzombie (`self.OwningZombie`))
  (`self.SourceWeapon`
    (:`then`
      (set `self.TraceStartLocation` (make `GameplayAbilityTargetingLocationInfo` "LiteralTransform" (`KismetMathLibrary.MakeTransform` (+ (`Actor.K2_GetActorLocation` _owningzombie) (* (`Actor.GetActorForwardVector` _owningzombie) 100.0)))))
      (`GSGATA_SphereTrace.Configure` :`self` (`self.SphereTraceActor`) :`InStartLocation` (`self.TraceStartLocation`) :`InTraceProfile` (struct :`Name` "EnemyAttack") :`bInShouldProduceTargetDataOnServer` true :`bInDebug` true :`InMaxRange` 0.0)
      (bind (_asynctaskproxy _data) (`GSAT_WaitTargetDataUsingActor.WaitTargetDataWithReusableActor` "None" "Instant" (`self.SphereTraceActor`) true)
        (:`then`
          (bind _asgsability_system_component (cast `GSAbilitySystemComponent` (`AbilitySystemBlueprintLibrary.GetAbilitySystemComponent` (`self.OwningZombie`))))
          (`GSAbilitySystemComponent.ExecuteGameplayCueLocal` _asgsability_system_component (struct :`TagName` "GameplayCue.Enemy.Zombie.Attack") (`AbilitySystemBlueprintLibrary.MakeGameplayCueParameters` 0.0 0.0 (struct) (struct) (struct) (struct) (struct) (0.0 0.0 0.0) (0.0 0.0 0.0) (`self.OwningZombie`))))
        (:`ValidData`
          (`self.HandleTargetData` _data))))
    (:`else`)))

(event `HandleTargetData`
  (params (TargetData :type "GameplayAbilityTargetDataHandle Structure"))
  (bind _returnvalue (`AbilitySystemBlueprintLibrary.AssignTagSetByCallerMagnitude` (`self.MakeOutgoingGameplayEffectSpec` "/Game/Survival/Blueprints/GameplayEffects/Enemy/Zombie/GE_ZombieMeleeDamage.GE_ZombieMeleeDamage_C") (struct :`TagName` "Data.Damage") (`self.Damage`)))
  (`self.K2_ApplyGameplayEffectSpecToTarget` _returnvalue TargetData)
  (bind _returnvalue_2 (`AbilitySystemBlueprintLibrary.GetEffectContext` _returnvalue))
  (`AbilitySystemBlueprintLibrary.EffectContextAddHitResult` _returnvalue_2 (`AbilitySystemBlueprintLibrary.GetHitResultFromTargetData` TargetData)))

(event `self.K2_OnEndAbility`
  (params (bWasCancelled :type Boolean))
  (bind _serverwaittargetdatatask (`self.ServerWaitTargetDataTask`)
    (:`then`
      (`GameplayTask.EndTask` _serverwaittargetdatatask))
    (:`else`
      _))
  (`self.K2_EndAbility` (`self.GA_ZombieMelee`)))

(fn `ActivationSetUp`
  (`self.SourceWeapon`
    (:`then`
      _)
    (:`else`
      (bind _asbp_zombie_weapon (cast `/Game/Survival/Blueprints/Weapon/Enemy/BP_ZombieWeapon` (`self.GetCurrentSourceObject`)))
      (set `self.SourceWeapon` _asbp_zombie_weapon)))
  (`self.OwningZombie`
    (:`then`
      _)
    (:`else`
      (bind _asbp_zombie (cast `/Game/Survival/Blueprints/Enemy/BP_Zombie` (`self.GetAvatarActorFromActorInfo`)))
      (set `self.OwningZombie` _asbp_zombie)))
  (`self.SphereTraceActor`
    (:`then`
      _)
    (:`else`
      (set `self.SphereTraceActor` (`/Game/Survival/Blueprints/Weapon/Enemy/BP_ZombieWeapon.SphereTraceActor` (`self.SourceWeapon`)))))
  (`self.GA_ZombieMelee`
    (:`then`
      _)
    (:`else`
      (bind _returnvalue (`GSBlueprintFunctionLibrary.GetPrimaryAbilityInstanceFromClass` (`self.GetAbilitySystemComponentFromActorInfo`) "/Game/Survival/Blueprints/GameplayAbilities/Enemy/Zombie/GA_ZombieMelee.GA_ZombieMelee_C"))
      (bind _asga_zombie_melee (cast `/Game/Survival/Blueprints/GameplayAbilities/Enemy/Zombie/GA_ZombieMelee` _returnvalue))
      (set `self.GA_ZombieMelee` _asga_zombie_melee)))
  (return))