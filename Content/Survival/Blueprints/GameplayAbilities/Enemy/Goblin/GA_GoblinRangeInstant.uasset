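; Goblin ranged attack ability that plays a montage and spits a slime ball at player 0 on the spit event.
; After a server-only net sync, it waits for client target data and runs an instant trace from the mouth socket using the weapon's reusable target actor.
; Target data spawns BP_SlimeBall carrying a SetByCaller damage effect spec.
; Ending also closes the target data task and the cached GA_GoblinRange ability.
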(event `self.K2_ActivateAbility`
  (`self.ActivationSetUp`)
  (`GSAT_PlayMontageForMeshAndWaitForEvent.PlayMontageForMeshAndWaitForEvent` "None" (`Character.Mesh` (`self.OwningGoblin`)) "/Game/ActionRPG/Animations/NPC/AM_Guardian_Attack02.AM_Guardian_Attack02" (struct :`GameplayTags` (struct :`(TagName` "Ability.Spit"))) 1.0 "None" true 1.0 true 0.0 0.0
    (:`OnCompleted`
      (`AbilityTask_NetworkSyncPoint.WaitNetSync` "BothWait"
        (:`OnSync`
          (`self.K2_EndAbility`))))
    (:`OnInterrupted`
      (`self.K2_CancelAbility` :!label _label))
    (:`OnCancelled`
      (goto _label))
    (:`EventReceived`
      (`AbilityTask_NetworkSyncPoint.WaitNetSync` "OnlyServerWait"
        (:`OnSync`
          (bind (_asynctaskproxy _data) (`GSAT_ServerWaitForClientTargetData.ServerWaitForClientTargetData` "None")
            (:`then`
              (set `self.ServerWaitTargetDataTask` _asynctaskproxy)
              (`self.SpitSlimeBall`))
            (:`ValidData`
              (`self.HandleTargetData` _data))))))))

(event `SpitSlimeBall`
  (bind _returnvalue_location (`KismetMathLibrary.BreakTransform` (`SceneComponent.GetSocketTransform` (`Character.Mesh` (`self.OwningGoblin`)) "SpitLocationSocket" "RTS_World")))
  (`self.SourceWeapon`
    (:`then`
      (set `self.TraceStartLocation` (make `GameplayAbilityTargetingLocationInfo` "LiteralTransform" (`KismetMathLibrary.MakeTransform` _returnvalue_location (`KismetMathLibrary.Conv_VectorToRotator` (- (`Actor.K2_GetActorLocation` (`GameplayStatics.GetPlayerPawn` 0)) _returnvalue_location))) null null null "SpitLocationSocket"))
      (`GSGATA_LineTrace.Configure` :`self` (`self.LineTraceActor`) :`InStartLocation` (`self.TraceStartLocation`) :`InTraceProfile` (struct :`Name` "EnemyAttack") :`bInShouldProduceTargetDataOnServer` true)
      (bind (_asynctaskproxy _data) (`GSAT_WaitTargetDataUsingActor.WaitTargetDataWithReusableActor` "None" "Instant" (`self.LineTraceActor`) true)
        (:`ValidData`
          (`self.HandleTargetData` _data))))
    (:`else`)))

(event `HandleTargetData`
  (params (TargetData :type "GameplayAbilityTargetDataHandle Structure"))
  (bind _owninggoblin (`self.OwningGoblin`))
  (bind (_bblockinghit _binitialoverlap _time _distance _location _impactpoint _normal _impactnormal _physmat _hitactor _hitcomponent _hitbonename _bonename _hititem _elementindex _faceindex _tracestart) (`GameplayStatics.BreakHitResult` (`AbilitySystemBlueprintLibrary.GetHitResultFromTargetData` TargetData)))
  (bind _returnvalue (`self.MakeEffectContainerSpec` (struct :`TagName` "Ability")))
  (`AbilitySystemBlueprintLibrary.AssignTagSetByCallerMagnitude` (`|GetArrayItem` (`.TargetGameplayEffectSpecs` (break `GSGameplayEffectContainerSpec` _returnvalue))) (struct :`TagName` "Data.Damage") (`self.Damage`))
  (`|SpawnActorFromClass` "/Game/Survival/Blueprints/Projectile/BP_SlimeBall.BP_SlimeBall_C" (`KismetMathLibrary.MakeTransform` _tracestart (`KismetMathLibrary.FindLookAtRotation` _tracestart _location)) "Undefined" "MultiplyWithRoot" _owninggoblin _returnvalue _owninggoblin))

(event `self.K2_OnEndAbility`
  (params (bWasCancelled :type Boolean))
  (bind _serverwaittargetdatatask (`self.ServerWaitTargetDataTask`)
    (:`then`
      (`GameplayTask.EndTask` _serverwaittargetdatatask))
    (:`else`
      _))
  (`self.K2_EndAbility` (`self.GA_GoblinRange`)))

(fn `ActivationSetUp`
  (`self.SourceWeapon`
    (:`then`
      _)
    (:`else`
      (bind _asbp_goblin_weapon (cast `/Game/Survival/Blueprints/Weapon/Enemy/BP_GoblinWeapon` (`self.GetCurrentSourceObject`)))
      (set `self.SourceWeapon` _asbp_goblin_weapon)))
  (`self.OwningGoblin`
    (:`then`
      _)
    (:`else`
      (bind _asbp_goblin (cast `/Game/Survival/Blueprints/Enemy/BP_Goblin` (`self.GetAvatarActorFromActorInfo`)))
      (set `self.OwningGoblin` _asbp_goblin)))
  (`self.LineTraceActor`
    (:`then`
      _)
    (:`else`
      (set `self.LineTraceActor` (`/Game/Survival/Blueprints/Weapon/Enemy/BP_GoblinWeapon.LineTraceActor` (`self.SourceWeapon`)))))
  (`self.GA_GoblinRange`
    (:`then`
      _)
    (:`else`
      (bind _returnvalue (`GSBlueprintFunctionLibrary.GetPrimaryAbilityInstanceFromClass` (`self.GetAbilitySystemComponentFromActorInfo`) "/Game/Survival/Blueprints/GameplayAbilities/Enemy/Goblin/GA_GoblinRange.GA_GoblinRange_C"))
      (bind _asga_goblin_range (cast `/Game/Survival/Blueprints/GameplayAbilities/Enemy/Goblin/GA_GoblinRange` _returnvalue))
      (set `self.GA_GoblinRange` _asga_goblin_range)))
  (return))