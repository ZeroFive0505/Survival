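; Goblin enemy melee attack ability that plays an attack montage and deals damage on the melee event.
; Activation caches the goblin, source weapon, reusable sphere trace actor and GA_GoblinMelee instance, which is ended alongside this ability.
; The montage event triggers a net sync, a server wait for client target data and an instant trace ahead of the capsule.
; Target data from either source receives GE_GoblinMeleeDamage via set-by-caller magnitude.
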(event `self.K2_ActivateAbility`
  (`self.ActivationSetUp`)
  (`GSAT_PlayMontageForMeshAndWaitForEvent.PlayMontageForMeshAndWaitForEvent` "None" (`Character.Mesh` (`self.OwningGoblin`)) "/Game/ActionRPG/Animations/NPC/AM_Guardian_Attack.AM_Guardian_Attack" (struct :`GameplayTags` (struct :`(TagName` "Ability.Melee"))) 1.0 "None" false 1.0 true 0.0 0.0
    (:`OnCompleted`
      (`AbilityTask_NetworkSyncPoint.WaitNetSync` "BothWait"
        (:`OnSync`
          (`self.K2_EndAbility`))))
    (:`OnInterrupted`
      (`self.K2_CancelAbility` :!label _label))
    (:`OnCancelled`
      (goto _label))
    (:`EventReceived`
      (`AbilityTask_NetworkSyncPoint.WaitNetSync` "OnlyServerWait"
        (:`OnSync`
          (bind (_asynctaskproxy _data) (`GSAT_ServerWaitForClientTargetData.ServerWaitForClientTargetData` "None")
            (:`then`
              (set `self.ServerWaitTargetDataTask` _asynctaskproxy)
              (`self.UseWeapon`))
            (:`ValidData`
              (`self.HandleTargetData` _data))))))))

(event `UseWeapon`
  (bind _owninggoblin (`self.OwningGoblin`))
  (set `self.TraceStartLocation` (make `GameplayAbilityTargetingLocationInfo` "LiteralTransform" (`KismetMathLibrary.MakeTransform` (+ (`Actor.K2_GetActorLocation` _owninggoblin) (* (`SceneComponent.GetForwardVector` (`Character.CapsuleComponent` _owninggoblin)) 50.0))) null null null "WeaponSocket"))
  (`GSGATA_SphereTrace.Configure` :`self` (`self.SphereTraceActor`) :`InStartLocation` (`self.TraceStartLocation`) :`InTraceProfile` (struct :`Name` "EnemyAttack") :`bInShouldProduceTargetDataOnServer` true :`bInDebug` true :`InMaxRange` 0.0)
  (bind (_asynctaskproxy _data) (`GSAT_WaitTargetDataUsingActor.WaitTargetDataWithReusableActor` "None" "Instant" (`self.SphereTraceActor`) true)
    (:`ValidData`
      (`self.HandleTargetData` _data))))

(event `HandleTargetData`
  (params (TargetData :type "GameplayAbilityTargetDataHandle Structure"))
  (bind _returnvalue (`AbilitySystemBlueprintLibrary.AssignTagSetByCallerMagnitude` (`self.MakeOutgoingGameplayEffectSpec` "/Game/Survival/Blueprints/GameplayEffects/Enemy/Goblin/GE_GoblinMeleeDamage.GE_GoblinMeleeDamage_C") (struct :`TagName` "Data.Damage") (`self.Damage`)))
  (`self.K2_ApplyGameplayEffectSpecToTarget` _returnvalue TargetData)
  (bind _returnvalue_2 (`AbilitySystemBlueprintLibrary.GetEffectContext` _returnvalue))
  (`AbilitySystemBlueprintLibrary.EffectContextAddHitResult` _returnvalue_2 (`AbilitySystemBlueprintLibrary.GetHitResultFromTargetData` TargetData)))

(event `self.K2_OnEndAbility`
  (params (bWasCancelled :type Boolean))
  (bind _serverwaittargetdatatask (`self.ServerWaitTargetDataTask`)
    (:`then`
      (`GameplayTask.EndTask` _serverwaittargetdatatask))
    (:`else`
      _))
  (`self.K2_EndAbility` (`self.GA_Melee`)))

(fn `ActivationSetUp`
  (`self.SourceWeapon`
    (:`then`
      _)
    (:`else`
      (bind _asbp_goblin_weapon (cast `/Game/Survival/Blueprints/Weapon/Enemy/BP_GoblinWeapon` (`self.GetCurrentSourceObject`)))
      (set `self.SourceWeapon` _asbp_goblin_weapon)))
  (`self.OwningGoblin`
    (:`then`
      _)
    (:`else`
      (bind _asbp_goblin (cast `/Game/Survival/Blueprints/Enemy/BP_Goblin` (`self.GetAvatarActorFromActorInfo`)))
      (set `self.OwningGoblin` _asbp_goblin)))
  (`self.SphereTraceActor`
    (:`then`
      _)
    (:`else`
      (set `self.SphereTraceActor` (`/Game/Survival/Blueprints/Weapon/Enemy/BP_GoblinWeapon.SphereTraceActor` (`self.SourceWeapon`)))))
  (`self.GA_Melee`
    (:`then`
      _)
    (:`else`
      (bind _returnvalue (`GSBlueprintFunctionLibrary.GetPrimaryAbilityInstanceFromClass` (`self.GetAbilitySystemComponentFromActorInfo`) "/Game/Survival/Blueprints/GameplayAbilities/Enemy/Goblin/GA_GoblinMelee.GA_GoblinMelee_C"))
      (bind _asga_goblin_melee (cast `/Game/Survival/Blueprints/GameplayAbilities/Enemy/Goblin/GA_GoblinMelee` _returnvalue))
      (set `self.GA_Melee` _asga_goblin_melee)))
  (return))