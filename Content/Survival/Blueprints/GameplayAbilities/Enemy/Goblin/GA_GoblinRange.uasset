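; Gameplay ability for the goblin's ranged attack, acting as the wrapper that triggers GA_GoblinRangeInstant.
; On activation it lazily caches the source goblin weapon, the instant ability's spec handle and instance, the weapon's line trace actor, and the owning goblin.
; It then activates the instant ability through BatchRPCTryActivateAbility without ending it immediately, following the GAS batched-RPC pattern.
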(event `self.K2_ActivateAbility`
  (`self.ActivationSetUp`)
  (`self.BatchRPCTryActivateAbility` (`self.InstantAbilityHandle`)))

(fn `ActivationSetUp`
  (`self.SourceWeapon`
    (:`then`
      _)
    (:`else`
      (bind _asbp_goblin_weapon (cast `/Game/Survival/Blueprints/Weapon/Enemy/BP_GoblinWeapon` (`self.GetCurrentSourceObject`)))
      (set `self.SourceWeapon` _asbp_goblin_weapon)))
  (if (not (`GSBlueprintFunctionLibrary.IsAbilitySpecHandleValid` (`self.InstantAbilityHandle`)))
    (bind _asgsability_system_component (cast `GSAbilitySystemComponent` (`self.GetAbilitySystemComponentFromActorInfo`)))
    (set `self.InstantAbilityHandle` (`GSAbilitySystemComponent.FindAbilitySpecHandleForClass` _asgsability_system_component "/Game/Survival/Blueprints/GameplayAbilities/Enemy/Goblin/GA_GoblinRangeInstant.GA_GoblinRangeInstant_C" (`self.SourceWeapon`))))
  (`self.InstantAbility`
    (:`then`
      _)
    (:`else`
      (bind _returnvalue (`GSBlueprintFunctionLibrary.GetPrimaryAbilityInstanceFromHandle` (`self.GetAbilitySystemComponentFromActorInfo`) (`self.InstantAbilityHandle`)))
      (bind _asga_goblin_range_instant (cast `/Game/Survival/Blueprints/GameplayAbilities/Enemy/Goblin/GA_GoblinRangeInstant` _returnvalue))
      (set `self.InstantAbility` _asga_goblin_range_instant)))
  (`self.LineTraceActor`
    (:`then`
      _)
    (:`else`
      (set `self.LineTraceActor` (`/Game/Survival/Blueprints/Weapon/Enemy/BP_GoblinWeapon.LineTraceActor` (`self.SourceWeapon`)))))
  (`self.OwningGoblin`
    (:`then`
      _)
    (:`else`
      (bind _asbp_goblin (cast `/Game/Survival/Blueprints/Enemy/BP_Goblin` (`self.GetAvatarActorFromActorInfo`)))
      (set `self.OwningGoblin` _asbp_goblin)))
  (return))