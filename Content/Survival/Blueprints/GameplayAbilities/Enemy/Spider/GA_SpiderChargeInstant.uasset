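; Spider enemy ability for the instant charge attack, which plays the charge montage and ends the companion GA_SpiderCharge ability when it finishes.
; On the montage's melee event, it net-syncs, listens for client target data and runs the weapon's reusable sphere trace actor just ahead of the spider.
; Target data from either path applies GE_SpiderChargeDamage with set-by-caller damage, then adds the hit result to the effect context.
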(event `self.K2_ActivateAbility`
  (`self.ActivationSetUp`)
  (`GSAT_PlayMontageForMeshAndWaitForEvent.PlayMontageForMeshAndWaitForEvent` "None" (`Character.Mesh` (`self.OwningSpider`)) "/Game/ActionRPG/Animations/Boss/AM_Spider_Charge.AM_Spider_Charge" (struct :`GameplayTags` (struct :`(TagName` "Ability.Melee"))) 1.0 "None" true 1.0 true 0.0 0.0
    (:`OnCompleted`
      (`AbilityTask_NetworkSyncPoint.WaitNetSync` "BothWait"
        (:`OnSync`
          (`self.K2_EndAbility`))))
    (:`OnInterrupted`
      (`self.K2_CancelAbility` :!label _label))
    (:`OnCancelled`
      (goto _label))
    (:`EventReceived`
      (`AbilityTask_NetworkSyncPoint.WaitNetSync` "OnlyServerWait"
        (:`OnSync`
          (bind (_asynctaskproxy _data) (`GSAT_ServerWaitForClientTargetData.ServerWaitForClientTargetData` "None")
            (:`then`
              (set `self.ServerWaitTargetDataTask` _asynctaskproxy)
              (`self.UseAbility`))
            (:`ValidData`
              (`self.HandleTargetData` _data))))))))

(event `HandleTargetData`
  (params (TargetData :type "GameplayAbilityTargetDataHandle Structure"))
  (bind _returnvalue (`AbilitySystemBlueprintLibrary.AssignTagSetByCallerMagnitude` (`self.MakeOutgoingGameplayEffectSpec` "/Game/Survival/Blueprints/GameplayEffects/Enemy/Spider/GE_SpiderChargeDamage.GE_SpiderChargeDamage_C") (struct :`TagName` "Data.Damage") (`self.Damage`)))
  (`self.K2_ApplyGameplayEffectSpecToTarget` _returnvalue TargetData)
  (bind _returnvalue_2 (`AbilitySystemBlueprintLibrary.GetEffectContext` _returnvalue))
  (`AbilitySystemBlueprintLibrary.EffectContextAddHitResult` _returnvalue_2 (`AbilitySystemBlueprintLibrary.GetHitResultFromTargetData` TargetData)))

(event `UseAbility`
  (bind _owningspider (`self.OwningSpider`))
  (set `self.TraceStartLocation` (make `GameplayAbilityTargetingLocationInfo` "LiteralTransform" (`KismetMathLibrary.MakeTransform` (+ (`Actor.K2_GetActorLocation` _owningspider) (* (`Actor.GetActorForwardVector` _owningspider) 200.0)))))
  (`GSGATA_SphereTrace.Configure` :`self` (`self.SphereTraceActor`) :`InStartLocation` (`self.TraceStartLocation`) :`InTraceProfile` (struct :`Name` "EnemyAttack") :`bInShouldProduceTargetDataOnServer` true :`bInDebug` true :`InMaxRange` 30.0 :`InTraceSphereRadius` 200.0)
  (bind (_asynctaskproxy _data) (`GSAT_WaitTargetDataUsingActor.WaitTargetDataWithReusableActor` "None" "Instant" (`self.SphereTraceActor`) true)
    (:`ValidData`
      (`self.HandleTargetData` _data))))

(event `self.K2_OnEndAbility`
  (params (bWasCancelled :type Boolean))
  (bind _serverwaittargetdatatask (`self.ServerWaitTargetDataTask`)
    (:`then`
      (`GameplayTask.EndTask` _serverwaittargetdatatask))
    (:`else`
      _))
  (`self.K2_EndAbility` (`self.GA_SpiderCharge`)))

(fn `ActivationSetUp`
  (`self.SourceWeapon`
    (:`then`
      _)
    (:`else`
      (bind _asbp_spider_weapon (cast `/Game/Survival/Blueprints/Weapon/Enemy/BP_SpiderWeapon` (`self.GetCurrentSourceObject`)))
      (set `self.SourceWeapon` _asbp_spider_weapon)))
  (`self.OwningSpider`
    (:`then`
      _)
    (:`else`
      (bind _asbp_spider (cast `/Game/Survival/Blueprints/Enemy/BP_Spider` (`self.GetAvatarActorFromActorInfo`)))
      (set `self.OwningSpider` _asbp_spider)))
  (`self.SphereTraceActor`
    (:`then`
      _)
    (:`else`
      (set `self.SphereTraceActor` (`/Game/Survival/Blueprints/Weapon/Enemy/BP_SpiderWeapon.SphereTraceActor` (`self.SourceWeapon`)))))
  (`self.GA_SpiderCharge`
    (:`then`
      _)
    (:`else`
      (bind _returnvalue (`GSBlueprintFunctionLibrary.GetPrimaryAbilityInstanceFromClass` (`self.GetAbilitySystemComponentFromActorInfo`) "/Game/Survival/Blueprints/GameplayAbilities/Enemy/Spider/GA_SpiderCharge.GA_SpiderCharge_C"))
      (bind _asga_spider_charge (cast `/Game/Survival/Blueprints/GameplayAbilities/Enemy/Spider/GA_SpiderCharge` _returnvalue))
      (set `self.GA_SpiderCharge` _asga_spider_charge)))
  (return))