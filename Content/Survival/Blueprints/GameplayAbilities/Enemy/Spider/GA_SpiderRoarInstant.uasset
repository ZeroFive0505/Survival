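; Gameplay ability for the spider enemy's instant roar attack, which damages targets in a forward fan and ends the GA_SpiderRoar ability when finished.
; A montage's roar event triggers three instant sphere traces (center and angled to each side) using the weapon's reusable target actor, plus a roar gameplay cue.
; Target data, produced on the server or received from the client, applies SetByCaller damage, with net syncs coordinating timing.
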(event `self.K2_ActivateAbility`
  (`self.ActivationSetUp`)
  (`GSAT_PlayMontageForMeshAndWaitForEvent.PlayMontageForMeshAndWaitForEvent` "None" (`Character.Mesh` (`self.OwningSpider`)) "/Game/ActionRPG/Animations/Boss/AM_Spider_Firewall.AM_Spider_Firewall" (struct :`GameplayTags` (struct :`(TagName` "Ability.Roar"))) 1.0 "None" true 1.0 true 0.0 0.0
    (:`OnCompleted`
      (`AbilityTask_NetworkSyncPoint.WaitNetSync` "BothWait"
        (:`OnSync`
          (`self.K2_EndAbility`))))
    (:`OnInterrupted`
      (`self.K2_CancelAbility` :!label _label))
    (:`OnCancelled`
      (goto _label))
    (:`EventReceived`
      (`AbilityTask_NetworkSyncPoint.WaitNetSync` "OnlyServerWait"
        (:`OnSync`
          (bind (_asynctaskproxy _data) (`GSAT_ServerWaitForClientTargetData.ServerWaitForClientTargetData` "None")
            (:`then`
              (set `self.ServerWaitTargetDataTask` _asynctaskproxy)
              (`self.UseAbility`))
            (:`ValidData`
              (`self.HandleTargetData` _data))))))))

(event `HandleTargetData`
  (params (TargetData :type "GameplayAbilityTargetDataHandle Structure"))
  (bind _returnvalue (`AbilitySystemBlueprintLibrary.AssignTagSetByCallerMagnitude` (`self.MakeOutgoingGameplayEffectSpec` "/Game/Survival/Blueprints/GameplayEffects/Enemy/Spider/GE_SpiderRoarDamage.GE_SpiderRoarDamage_C") (struct :`TagName` "Data.Damage") (`self.Damage`)))
  (`self.K2_ApplyGameplayEffectSpecToTarget` _returnvalue TargetData)
  (bind _returnvalue_2 (`AbilitySystemBlueprintLibrary.GetEffectContext` _returnvalue))
  (`AbilitySystemBlueprintLibrary.EffectContextAddHitResult` _returnvalue_2 (`AbilitySystemBlueprintLibrary.GetHitResultFromTargetData` TargetData)))

(event `self.K2_OnEndAbility`
  (params (bWasCancelled :type Boolean))
  (bind _serverwaittargetdatatask (`self.ServerWaitTargetDataTask`)
    (:`then`
      (`GameplayTask.EndTask` _serverwaittargetdatatask))
    (:`else`
      _))
  (`self.K2_EndAbility` (`self.GA_SpiderRoar`)))

(event `UseAbility`
  (bind _owningspider (`self.OwningSpider`))
  (bind _owningspider_2 (`self.OwningSpider`))
  (bind _owningspider_3 (`self.OwningSpider`))
  (bind _owningspider_4 (`self.OwningSpider`))
  (bind _returnvalue (`SceneComponent.GetForwardVector` (`Character.CapsuleComponent` _owningspider_4)))
  (bind _returnvalue_2 (`KismetMathLibrary.RotateAngleAxis` (`SceneComponent.GetForwardVector` (`Character.CapsuleComponent` _owningspider_3)) -25.0 (0.0 0.0 1.0)))
  (bind _returnvalue_3 (`KismetMathLibrary.RotateAngleAxis` (`SceneComponent.GetForwardVector` (`Character.CapsuleComponent` _owningspider)) 25.0 (0.0 0.0 1.0)))
  (`|ExecutionSequence`
    (:`then_0`
      (set `self.TraceStartLocation` (make `GameplayAbilityTargetingLocationInfo` "LiteralTransform" (`KismetMathLibrary.MakeTransform` (+ (`Actor.K2_GetActorLocation` _owningspider_4) (* _returnvalue 200.0)) (`KismetMathLibrary.Conv_VectorToRotator` _returnvalue))))
      (`GSGATA_SphereTrace.Configure` :`self` (`self.SphereTraceActor`) :`InStartLocation` (`self.TraceStartLocation`) :`InTraceProfile` (struct :`Name` "EnemyAttack") :`bInShouldProduceTargetDataOnServer` true :`bInDebug` true :`InMaxRange` 1000.0)
      (bind (_asynctaskproxy _data) (`GSAT_WaitTargetDataUsingActor.WaitTargetDataWithReusableActor` "None" "Instant" (`self.SphereTraceActor`) true)
        (:`ValidData`
          (`self.HandleTargetData` _data))))
    (:`then_1`
      (set `self.TraceStartLocation` (make `GameplayAbilityTargetingLocationInfo` "LiteralTransform" (`KismetMathLibrary.MakeTransform` (+ (`Actor.K2_GetActorLocation` _owningspider) (* _returnvalue_3 200.0)) (`KismetMathLibrary.Conv_VectorToRotator` _returnvalue_3))))
      (`GSGATA_SphereTrace.Configure` :`self` (`self.SphereTraceActor`) :`InStartLocation` (`self.TraceStartLocation`) :`InTraceProfile` (struct :`Name` "EnemyAttack") :`bInShouldProduceTargetDataOnServer` true :`bInDebug` true :`InMaxRange` 1000.0)
      (bind (_asynctaskproxy_2 _data_2) (`GSAT_WaitTargetDataUsingActor.WaitTargetDataWithReusableActor` "None" "Instant" (`self.SphereTraceActor`) true)
        (:`ValidData`
          (`self.HandleTargetData` _data_2))))
    (:`then_2`
      (set `self.TraceStartLocation` (make `GameplayAbilityTargetingLocationInfo` "LiteralTransform" (`KismetMathLibrary.MakeTransform` (+ (`Actor.K2_GetActorLocation` _owningspider_3) (* _returnvalue_2 200.0)) (`KismetMathLibrary.Conv_VectorToRotator` _returnvalue_2))))
      (`GSGATA_SphereTrace.Configure` :`self` (`self.SphereTraceActor`) :`InStartLocation` (`self.TraceStartLocation`) :`InTraceProfile` (struct :`Name` "EnemyAttack") :`bInShouldProduceTargetDataOnServer` true :`bInDebug` true :`InMaxRange` 1000.0)
      (bind (_asynctaskproxy_3 _data_3) (`GSAT_WaitTargetDataUsingActor.WaitTargetDataWithReusableActor` "None" "Instant" (`self.SphereTraceActor`) true)
        (:`ValidData`
          (`self.HandleTargetData` _data_3))))
    (:`then_3`
      (`self.K2_ExecuteGameplayCueWithParams` (struct :`TagName` "GameplayCue.Ability.Roar") (`AbilitySystemBlueprintLibrary.MakeGameplayCueParameters` 0.0 0.0 (struct) (struct) (struct) (struct) (struct) (`Actor.K2_GetActorLocation` _owningspider_2) (0.0 0.0 0.0) _owningspider_2 null (`AbilitySystemBlueprintLibrary.GetAbilitySystemComponent` _owningspider_2))))))

(fn `ActivationSetUp`
  (`self.SourceWeapon`
    (:`then`
      _)
    (:`else`
      (bind _asbp_spider_weapon (cast `/Game/Survival/Blueprints/Weapon/Enemy/BP_SpiderWeapon` (`self.GetCurrentSourceObject`)))
      (set `self.SourceWeapon` _asbp_spider_weapon)))
  (`self.OwningSpider`
    (:`then`
      _)
    (:`else`
      (bind _asbp_spider (cast `/Game/Survival/Blueprints/Enemy/BP_Spider` (`self.GetAvatarActorFromActorInfo`)))
      (set `self.OwningSpider` _asbp_spider)))
  (`self.SphereTraceActor`
    (:`then`
      _)
    (:`else`
      (set `self.SphereTraceActor` (`/Game/Survival/Blueprints/Weapon/Enemy/BP_SpiderWeapon.SphereTraceActor` (`self.SourceWeapon`)))))
  (`self.GA_SpiderRoar`
    (:`then`
      _)
    (:`else`
      (bind _returnvalue (`GSBlueprintFunctionLibrary.GetPrimaryAbilityInstanceFromClass` (`self.GetAbilitySystemComponentFromActorInfo`) "/Game/Survival/Blueprints/GameplayAbilities/Enemy/Spider/GA_SpiderRoar.GA_SpiderRoar_C"))
      (bind _asga_spider_roar (cast `/Game/Survival/Blueprints/GameplayAbilities/Enemy/Spider/GA_SpiderRoar` _returnvalue))
      (set `self.GA_SpiderRoar` _asga_spider_roar)))
  (return))