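; Spider enemy roar gameplay ability that acts as the outer wrapper for GA_SpiderRoarInstant.
; On activation, ActivationSetUp lazily caches the source spider weapon, the instant ability's spec handle and instance, the owning spider and the weapon's sphere trace actor.
; It then triggers the instant ability through a batched RPC without ending it immediately, following the GASShooter-style split between primary and instant abilities.
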(event `self.K2_ActivateAbility`
  (`self.ActivationSetUp`)
  (`self.BatchRPCTryActivateAbility` (`self.InstantAbilityHandle`)))

(event `self.K2_OnEndAbility`
  (params (bWasCancelled :type Boolean))
  (`parent.K2_OnEndAbility` bWasCancelled))

(fn `ActivationSetUp`
  (`self.SourceWeapon`
    (:`then`
      _)
    (:`else`
      (bind _asbp_spider_weapon (cast `/Game/Survival/Blueprints/Weapon/Enemy/BP_SpiderWeapon` (`self.GetCurrentSourceObject`)))
      (set `self.SourceWeapon` _asbp_spider_weapon)))
  (if (not (`GSBlueprintFunctionLibrary.IsAbilitySpecHandleValid` (`self.InstantAbilityHandle`)))
    (bind _asgsability_system_component (cast `GSAbilitySystemComponent` (`self.GetAbilitySystemComponentFromActorInfo`)))
    (set `self.InstantAbilityHandle` (`GSAbilitySystemComponent.FindAbilitySpecHandleForClass` _asgsability_system_component "/Game/Survival/Blueprints/GameplayAbilities/Enemy/Spider/GA_SpiderRoarInstant.GA_SpiderRoarInstant_C" (`self.SourceWeapon`))))
  (`self.InstantAbility`
    (:`then`
      _)
    (:`else`
      (bind _returnvalue (`GSBlueprintFunctionLibrary.GetPrimaryAbilityInstanceFromHandle` (`self.GetAbilitySystemComponentFromActorInfo`) (`self.InstantAbilityHandle`)))
      (bind _asga_spider_roar_instant (cast `/Game/Survival/Blueprints/GameplayAbilities/Enemy/Spider/GA_SpiderRoarInstant` _returnvalue))
      (set `self.InstantAbility` _asga_spider_roar_instant)))
  (`self.OwningSpider`
    (:`then`
      _)
    (:`else`
      (bind _asbp_spider (cast `/Game/Survival/Blueprints/Enemy/BP_Spider` (`self.GetAvatarActorFromActorInfo`)))
      (set `self.OwningSpider` _asbp_spider)))
  (`self.SphereTraceActor`
    (:`then`
      _)
    (:`else`
      (set `self.SphereTraceActor` (`/Game/Survival/Blueprints/Weapon/Enemy/BP_SpiderWeapon.SphereTraceActor` (`self.SourceWeapon`)))))
  (return))