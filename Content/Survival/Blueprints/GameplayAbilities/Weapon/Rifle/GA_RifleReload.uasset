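; Gameplay ability that reloads a survivor's rifle, activatable only when the clip is not full and reserve ammo remains.
; It plays third-person and non-replicated first-person montages, with the latter's reload event triggering the ammo transfer after a server-only net sync.
; The transfer is capped by reserve, which a SetByCaller gameplay effect reduces, while the weapon's clip is set directly.
; Completion ends the ability after a two-way sync; interruption cancels it.
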(event `self.K2_ActivateAbility`
  (bind _sourceweapoon (`self.SourceWeapoon`))
  (bind _returnvalue (`GSSurvivor.GetPrimaryReserveAmmo` (`self.OwningSurvivor`)))
  (`self.ActivationSetUp`)
  (`GSAT_PlayMontageForMeshAndWaitForEvent.PlayMontageForMeshAndWaitForEvent` "None" (`GSSurvivor.GetThirdPersonMesh` (`self.OwningSurvivor`)) "/Game/ShooterGame/Animations/TTP_Animations/Reload_Montage.Reload_Montage" (struct) 1.0 "None" false 1.0 true 0.0 0.0
    (:`then`
      (`GSAT_PlayMontageForMeshAndWaitForEvent.PlayMontageForMeshAndWaitForEvent` "None" (`GSSurvivor.GetFirstPersonMesh` (`self.OwningSurvivor`)) "/Game/ShooterGame/Animations/FPP_Animations/HeroFPP_RifleReload_Montage.HeroFPP_RifleReload_Montage" (struct :`GameplayTags` (struct :`(TagName` "Ability.Weapon.Reload"))) 1.0 "None" false 1.0 false 0.0 0.0
        (:`OnCompleted`
          (`AbilityTask_NetworkSyncPoint.WaitNetSync` "BothWait"
            (:`OnSync`
              (`self.K2_EndAbility`))))
        (:`OnInterrupted`
          (`self.K2_CancelAbility` :!label _label))
        (:`OnCancelled`
          (goto _label))
        (:`EventReceived`
          (`AbilityTask_NetworkSyncPoint.WaitNetSync` "OnlyServerWait"
            (:`OnSync`
              (bind _output_get (set `self.AmountWeWantToReload` (- (`GSWeapon.GetMaxPrimaryClipAmmo` _sourceweapoon) (`GSWeapon.GetPrimaryClipAmmo` _sourceweapoon))))
              (if (<= _output_get _returnvalue)
                (set `self.AmountWeCanReload` _output_get)
                (else
                  (set `self.AmountWeCanReload` _returnvalue)))
              (bind _returnvalue_2 (`self.MakeEffectContainerSpec` (struct :`TagName` "Ability")))
              (`AbilitySystemBlueprintLibrary.AssignTagSetByCallerMagnitude` (`|GetArrayItem` (`.TargetGameplayEffectSpecs` (break `GSGameplayEffectContainerSpec` _returnvalue_2))) (struct :`TagName` "Data.ReloadAmount.Reserve") (`KismetMathLibrary.Conv_IntToDouble` (* (`self.AmountWeCanReload`) -1)))
              (`self.ApplyEffectContainerSpec` _returnvalue_2)
              (`GSWeapon.SetPrimaryClipAmmo` (`self.SourceWeapoon`) (+ (`GSWeapon.GetPrimaryClipAmmo` (`self.SourceWeapoon`)) (`self.AmountWeCanReload`))))))))))

(fn `ActivationSetUp`
  (`self.SourceWeapoon`
    (:`then`
      _)
    (:`else`
      (bind _asgsweapon (cast `GSWeapon` (`self.GetCurrentSourceObject`)))
      (set `self.SourceWeapoon` _asgsweapon)))
  (`self.OwningSurvivor`
    (:`then`
      _)
    (:`else`
      (bind _asbp_survivor (cast `/Game/Survival/Blueprints/Characters/BP_Survivor` (`self.GetAvatarActorFromActorInfo`)))
      (set `self.OwningSurvivor` _asbp_survivor)))
  (return))

(fn `K2_CanActivateAbility`
  (params (ActorInfo :type "GameplayAbilityActorInfo Structure") (Handle :type "GameplayAbilitySpecHandle Structure"))
  (returns (RelevantTags :type "GameplayTagContainer Structure") (ReturnValue :type Boolean))
  (bind _asbp_survivor (cast `/Game/Survival/Blueprints/Characters/BP_Survivor` (`.AvatarActor` (break `GameplayAbilityActorInfo` ActorInfo))))
  (return (struct) (and (< (`GSSurvivor.GetPrimaryClipAmmo` _asbp_survivor) (`GSSurvivor.GetMaxPrimaryClipAmmo` _asbp_survivor)) (> (`GSSurvivor.GetPrimaryReserveAmmo` _asbp_survivor) 0))))