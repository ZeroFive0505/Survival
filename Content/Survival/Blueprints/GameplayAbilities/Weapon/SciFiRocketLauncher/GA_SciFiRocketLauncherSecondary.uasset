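; Secondary-fire gameplay ability for the sci-fi rocket launcher: hold to aim down sights and lock on, firing homing rockets at multiple targets.
; A reusable sphere-trace actor gathers ammo-capped targets locally, while the server awaits replicated target data.
; Confirmed data drives staggered shots with server-spawned projectiles and local fire cues, then targeting restarts while ammo remains.
; Custom cost uses clip ammo and can trigger reload; ending restores camera, HUD and aim state.
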(event `ZoomBackAndFinishAbility`
  (bind _owningsurvivor (`self.OwningSurvivor`))
  (bind _asynctaskproxy (`GSAT_WaitChangeFOV.WaitChangeFOV` "None" (`GSSurvivor.FirstPersonCamera` _owningsurvivor) (`GSSurvivor.Default1PFOV` _owningsurvivor) 0.05)
    (:`then`
      (set `self.ZoomResetTask` _asynctaskproxy)
      (bind _returnvalue (`self.BP_ApplyGameplayEffectToOwner` (`self.GE_AimingRemoval_Class`) (`self.GetAbilityLevel`)))
      (set `self.GE_AimingRemoval` _returnvalue))
    (:`OnTargetFOVReached`
      (`self.K2_EndAbility`))))

(event `self.K2_ActivateAbility`
  (set `self.GE_AimingRemoval` (struct))
  (`self.ActivationSetUp`)
  (bind _returnvalue (`self.BP_ApplyGameplayEffectToOwner` (`self.GE_Aiming_Class`) (`self.GetAbilityLevel`)))
  (set `self.GE_Aiming` _returnvalue)
  (bind _asynctaskproxy (`GSAT_WaitChangeFOV.WaitChangeFOV` "None" (`GSSurvivor.FirstPersonCamera` (`self.OwningSurvivor`)) (`self.TargetingFOV`) 0.1)
    (:`then`
      (set `self.ZoomInTask` _asynctaskproxy)
      (set `SpringArmComponent.TargetArmLength` 100.0 (`GSSurvivor.ThirdPersonCameraBoom` (`self.OwningSurvivor`)))
      (bind _asgscharacter_movement_component (cast `GSCharacterMovementComponent` (`.MovementComponent` (break `GameplayAbilityActorInfo` (`self.GetActorInfo`)))))
      (`GSCharacterMovementComponent.StartAimDownSights` _asgscharacter_movement_component)
      (`AbilityTask_WaitInputRelease.WaitInputRelease` true
        (:`then`
          (bind (_asynctaskproxy_2 _data) (`GSAT_ServerWaitForClientTargetData.ServerWaitForClientTargetData` "None")
            (:`then`
              (set `self.ServerWaitTargetDataTask` _asynctaskproxy_2)
              (`self.StartTargeting`)
              (set `GSWeapon.StatusText` "Homing" (`self.SourceWeapon`))
              (bind _playercontroller (`self.PlayerController`)
                (:`then`
                  (`GSPlayerController.SetEquippedWeaponStatusText` _playercontroller (`GSWeapon.StatusText` (`self.SourceWeapon`))))
                (:`else`)))
            (:`ValidData`
              (`self.HandleTargetData` _data))))
        (:`OnRelease`
          (`self.ZoomBackAndFinishAbility`))))))

(event `StartTargeting`
  (if (`Controller.IsLocalPlayerController` (`.PlayerController` (break `GameplayAbilityActorInfo` (`self.GetActorInfo`))))
    (bind _aiminghudreticle (`self.AimingHUDReticle`)
      (:`then`
        (`self.SetHUDReticle` _aiminghudreticle))
      (:`else`
        _))
    (`self.SourceWeapon`
      (:`then`
        (if (`GSSurvivor.IsInFirstPersonPerspective` (`self.OwningSurvivor`))
          (set `self.TraceStartLocation` (make `GameplayAbilityTargetingLocationInfo` "SocketTransform" "0.000000,0.000000,0.000000|0.000000,0.000000,-0.000000|1.000000,1.000000,1.000000" null (`self.Weapon1PMesh`) null "MuzzleFlashSocket"))
          (set `self.TraceFromPlayerViewPoint` true)
          (else
            (set `self.TraceStartLocation` (make `GameplayAbilityTargetingLocationInfo` "SocketTransform" "0.000000,0.000000,0.000000|0.000000,0.000000,-0.000000|1.000000,1.000000,1.000000" null (`self.Weapon3PMesh`) null "MuzzleFlashSocket"))
            (set `self.TraceFromPlayerViewPoint` false)))
        (bind _sourceweapon (`self.SourceWeapon`)
          (:`then`
            (`GSGATA_SphereTrace.Configure` :`self` (`self.SphereTraceTargetActor`) :`InStartLocation` (`self.TraceStartLocation`) :`InTraceProfile` (struct :`Name` "Projectile") :`InReticleClass` "/Game/Survival/Blueprints/UI/Reticles/BP_TargetLockOnReticleActor.BP_TargetLockOnReticleActor_C" :`bInUsePersistentHitResults` true :`bInTraceFromPlayerViewPoint` (`self.TraceFromPlayerViewPoint`) :`InMaxRange` (`self.MaxRange`) :`InMaxHitResultsPerTrace` (`KismetMathLibrary.Min` (`GSWeapon.GetPrimaryClipAmmo` _sourceweapon) (`self.MaxTargets`)))
            (bind (_asynctaskproxy _data) (`GSAT_WaitTargetDataUsingActor.WaitTargetDataWithReusableActor` "None" "UserConfirmed" (`self.SphereTraceTargetActor`) true)
              (:`then`
                (set `self.WaitTargetDataWithActorTask` _asynctaskproxy))
              (:`ValidData`
                (`self.HandleTargetData` _data))
              (:`Cancelled`
                (`self.ZoomBackAndFinishAbility`))))
          (:`else`)))
      (:`else`
        (`KismetSystemLibrary.PrintString` "Error: GA_SciFiRocketLauncherSecondary StartTargeting Launcher is null")))))

(event `HandleTargetData`
  (params (TargetData :type "GameplayAbilityTargetDataHandle Structure"))
  (bind _owningsurvivor (`self.OwningSurvivor`))
  (bind (_asynctaskproxy _actionnumber) (`AbilityTask_Repeat.RepeatAction` (`self.TimeBetweenFastRockets`) (`KismetMathLibrary.Min` (`AbilitySystemBlueprintLibrary.GetDataCountFromTargetData` TargetData) (`self.MaxTargets`)))
    (:`then`
      (set `self.FireRocketRepeatActionTask` _asynctaskproxy))
    (:`OnPerformAction`
      (bind _asgscharacter (cast `GSCharacter` (`.HitActor` (`GameplayStatics.BreakHitResult` (`AbilitySystemBlueprintLibrary.GetHitResultFromTargetData` TargetData _actionnumber)))))
      (if (`GSCharacter.IsAlive` _asgscharacter)
        (bind _returnvalue (`self.K2_CommitAbilityCost` false))
        (if _returnvalue
          (`self.PlayFireMontage`)
          (bind _returnvalue_2 (`self.MakeEffectContainerSpec` (struct :`TagName` "Ability")))
          (`AbilitySystemBlueprintLibrary.AssignTagSetByCallerMagnitude` (`|GetArrayItem` (`.TargetGameplayEffectSpecs` (break `GSGameplayEffectContainerSpec` _returnvalue_2))) (struct :`TagName` "Data.Damage") (`self.RocketDamage`))
          (if (`Actor.HasAuthority` (`self.OwningSurvivor`))
            (bind (_bblockinghit _binitialoverlap _time _distance _location _impactpoint _normal _impactnormal _physmat _hitactor _hitcomponent _hitbonename _bonename _hititem _elementindex _faceindex _tracestart) (`GameplayStatics.BreakHitResult` (`AbilitySystemBlueprintLibrary.GetHitResultFromTargetData` TargetData _actionnumber)))
            (bind _returnvalue_3 (`KismetMathLibrary.FindLookAtRotation` _tracestart _location))
            (`|SpawnActorFromClass` "/Game/Survival/Blueprints/Projectile/BP_SciFiRocketLauncherProjectile.BP_SciFiRocketLauncherProjectile_C" (`KismetMathLibrary.MakeTransform` _tracestart _returnvalue_3) "AlwaysSpawn" "OverrideRootScale" _owningsurvivor _returnvalue_2 true _hitactor _owningsurvivor))
          (if (`Pawn.IsLocallyControlled` (`self.OwningSurvivor`))
            (`GSAbilitySystemComponent.ExecuteGameplayCueLocal` (`self.ASC`) (struct :`TagName` "GameplayCue.Weapon.SciFiRocketLauncher.Fire") (`AbilitySystemBlueprintLibrary.MakeGameplayCueParameters` 0.0 0.0 (struct) (struct) (struct) (struct) (struct) _location (`KismetMathLibrary.GetForwardVector` _returnvalue_3) (`self.OwningSurvivor`))))
          (set `self.TimeOfLastShot` (`GameplayStatics.GetTimeSeconds`))
          (else
            (`self.ZoomBackAndFinishAbility`)))))
    (:`OnFinished`
      (bind _returnvalue_4 (`self.K2_CheckAbilityCost`))
      (if _returnvalue_4
        (if (`Pawn.IsLocallyControlled` (`self.OwningSurvivor`))
          (bind _waittargetdatawithactortask (`self.WaitTargetDataWithActorTask`)
            (:`then`
              (`GameplayTask.EndTask` _waittargetdatawithactortask))
            (:`else`
              _))
          (`AbilityTask_WaitDelay.WaitDelay` (`self.TimeToStartTargetingAgain`)
            (:`OnFinish`
              (`self.StartTargeting`))))
        (else
          (`self.ZoomBackAndFinishAbility`))))))

(event `PlayFireMontage`
  (bind _returnvalue (`self.GetAbilitySystemComponentFromActorInfo`))
  (bind _returnvalue_2 (`GSSurvivor.GetFirstPersonMesh` (`self.OwningSurvivor`)))
  (if (and (`GameplayTagAssetInterface.HasMatchingGameplayTag` _returnvalue (struct :`TagName` "Weapon.RocketLauncher.Aiming")) (not (`GameplayTagAssetInterface.HasMatchingGameplayTag` _returnvalue (struct :`TagName` "Weapon.RocketLauncher.AimingRemoval"))))
    (`GSAT_PlayMontageForMeshAndWaitForEvent.PlayMontageForMeshAndWaitForEvent` "None" _returnvalue_2 "/Game/ShooterGame/Animations/FPP_Animations/FPP_LauncherAimFire_Montage.FPP_LauncherAimFire_Montage" (struct) 1.0 "None" false 1.0 false)
    (else
      (`GSAT_PlayMontageForMeshAndWaitForEvent.PlayMontageForMeshAndWaitForEvent` "None" _returnvalue_2 "/Game/ShooterGame/Animations/FPP_Animations/HeroFPP_LauncherFire_Montage.HeroFPP_LauncherFire_Montage" (struct) 1.0 "None" false 1.0 false))))

(event `self.K2_OnEndAbility`
  (params (bWasCancelled :type Boolean))
  (bind _owningsurvivor (`self.OwningSurvivor`))
  (bind _owningsurvivor_2 (`self.OwningSurvivor`))
  (set `GSWeapon.StatusText` "Default" (`self.SourceWeapon`))
  (bind _playercontroller (`self.PlayerController`)
    (:`then`
      (`GSPlayerController.SetEquippedWeaponStatusText` _playercontroller (`GSWeapon.StatusText` (`self.SourceWeapon`))))
    (:`else`
      _))
  (`self.ResetHUDReticle`)
  (bind _waittargetdatawithactortask (`self.WaitTargetDataWithActorTask`)
    (:`then`
      (`GameplayTask.EndTask` _waittargetdatawithactortask))
    (:`else`
      _))
  (bind _serverwaittargetdatatask (`self.ServerWaitTargetDataTask`)
    (:`then`
      (`GameplayTask.EndTask` _serverwaittargetdatatask))
    (:`else`
      _))
  (bind _returnvalue (`AbilitySystemBlueprintLibrary.GetActiveGameplayEffectStackCount` (`self.GE_AimingRemoval`)))
  (if (not (> _returnvalue 0))
    (bind _returnvalue_2 (`self.BP_ApplyGameplayEffectToOwner` (`self.GE_AimingRemoval_Class`) (`self.GetAbilityLevel`)))
    (set `self.GE_AimingRemoval` _returnvalue_2))
  (`self.BP_RemoveGameplayEffectFromOwnerWithHandle` (`self.GE_Aiming`))
  (`self.BP_RemoveGameplayEffectFromOwnerWithHandle` (`self.GE_AimingRemoval`))
  (bind _zoomintask (`self.ZoomInTask`)
    (:`then`
      (`GameplayTask.EndTask` _zoomintask))
    (:`else`
      _))
  (bind _zoomresettask (`self.ZoomResetTask`)
    (:`then`
      (`GameplayTask.EndTask` _zoomresettask))
    (:`else`
      _))
  (`CameraComponent.SetFieldOfView` (`GSSurvivor.FirstPersonCamera` _owningsurvivor) (`GSSurvivor.Default1PFOV` _owningsurvivor))
  (set `SpringArmComponent.TargetArmLength` (`GSSurvivor.StartingThirdPersonCameraBoomArmLength` _owningsurvivor_2) (`GSSurvivor.ThirdPersonCameraBoom` _owningsurvivor_2))
  (bind _asgscharacter_movement_component (cast `GSCharacterMovementComponent` (`.MovementComponent` (break `GameplayAbilityActorInfo` (`self.GetActorInfo`)))))
  (`GSCharacterMovementComponent.StopAimDownSights` _asgscharacter_movement_component))

(fn `ActivationSetUp`
  (bind (_returnvalue_owneractor _returnvalue_avataractor _returnvalue_playercontroller) (break `GameplayAbilityActorInfo` (`self.GetActorInfo`)))
  (`self.OwningSurvivor`
    (:`then`
      _)
    (:`else`
      (bind _asbp_survivor (cast `/Game/Survival/Blueprints/Characters/BP_Survivor` (`self.GetAvatarActorFromActorInfo`)))
      (set `self.OwningSurvivor` _asbp_survivor)))
  (`self.SourceWeapon`
    (:`then`
      _)
    (:`else`
      (bind _asgsweapon (cast `GSWeapon` (`self.GetCurrentSourceObject`)))
      (set `self.SourceWeapon` _asgsweapon)))
  (`self.Weapon1PMesh`
    (:`then`
      _)
    (:`else`
      (set `self.Weapon1PMesh` (`GSWeapon.GetWeaponMesh1P` (`self.SourceWeapon`)))))
  (`self.Weapon3PMesh`
    (:`then`
      _)
    (:`else`
      (set `self.Weapon3PMesh` (`GSWeapon.GetWeaponMesh3P` (`self.SourceWeapon`)))))
  (`self.ASC`
    (:`then`
      _)
    (:`else`
      (bind _asgsability_system_component (cast `GSAbilitySystemComponent` (`self.GetAbilitySystemComponentFromActorInfo`)))
      (set `self.ASC` _asgsability_system_component)))
  (`self.SphereTraceTargetActor`
    (:`then`
      _)
    (:`else`
      (bind _returnvalue (`GSWeapon.GetSphereTraceTargetActor` (`self.SourceWeapon`)))
      (set `self.SphereTraceTargetActor` _returnvalue)))
  (`self.PlayerController`
    (:`then`
      _)
    (:`else`
      (bind _asgsplayer_controller (cast `GSPlayerController` _returnvalue_playercontroller)
        (:`then`
          (set `self.PlayerController` _asgsplayer_controller))
        (:`CastFailed`
          _))))
  (return))

(fn `GSApplyCost`
  (params (Handle :type "GameplayAbilitySpecHandle Structure") (ActorInfo :type "GameplayAbilityActorInfo Structure (by ref)") (ActivationInfo :type "GameplayAbilityActivationInfo Structure"))
  (bind _asgsweapon (cast `GSWeapon` (`self.BP_GetSourceObject` Handle ActorInfo)))
  (if (not (`GSWeapon.HasInfiniteAmmo` _asgsweapon))
    (`GSWeapon.SetPrimaryClipAmmo` _asgsweapon (- (`GSWeapon.GetPrimaryClipAmmo` _asgsweapon) (`self.AmmoCost`)))
    (return)))

(fn `GSCheckCost`
  (params (Handle :type "GameplayAbilitySpecHandle Structure") (ActorInfo :type "GameplayAbilityActorInfo Structure (by ref)"))
  (returns (ReturnValue :type Boolean))
  (bind (_owneractor _avataractor _playercontroller _abilitysystemcomponent) (break `GameplayAbilityActorInfo` (`local.ActorInfo`)))
  (bind _asgsweapon (cast `GSWeapon` (`self.BP_GetSourceObject` Handle ActorInfo)))
  (if (and (or (>= (`GSWeapon.PrimaryClipAmmo` _asgsweapon) (`self.AmmoCost`)) (`GSWeapon.HasInfiniteAmmo` _asgsweapon)) (`parent.GSCheckCost` (`local.Handle`) (`local.ActorInfo`)))
    (return true)
    (else
      (bind _returnvalue (`GSBlueprintFunctionLibrary.IsPrimaryAbilityInstanceActive` _abilitysystemcomponent (`local.Handle`)))
      (if (not _returnvalue)
        (`AbilitySystemComponent.TryActivateAbilitiesByTag` _abilitysystemcomponent (`BlueprintGameplayTagLibrary.MakeGameplayTagContainerFromArray` (`|MakeArray` (struct :`TagName` "Ability.Weapon.Reload") :!type "GameplayTag Structure")) true))
      (return false))))

(fn `K2_CanActivateAbility`
  (params (ActorInfo :type "GameplayAbilityActorInfo Structure") (Handle :type "GameplayAbilitySpecHandle Structure"))
  (returns (RelevantTags :type "GameplayTagContainer Structure") (ReturnValue :type Boolean))
  (if (>= (`KismetMathLibrary.Abs` (- (`GameplayStatics.GetTimeSeconds`) (`self.TimeOfLastShot`))) (`self.TimeBetweenShots`))
    (return (struct) true)
    (else
      (return (struct :`GameplayTags` (struct :`(TagName` "Activation.Fail.OnCooldown"))) false))))