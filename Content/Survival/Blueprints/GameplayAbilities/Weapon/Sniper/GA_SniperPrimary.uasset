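; Sniper primary-fire Gameplay Ability that acts as a wrapper, delegating the shot to GA_SniperPrimaryInstant.
; On activation it caches the source weapon and instant ability, waits one frame (or briefly longer when sprinting), then ends itself after triggering that ability through a batched RPC.
; Its cost check requires enough clip ammo or infinite ammo plus the parent check, and on failure attempts a reload unless this ability is already active.
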(event `self.K2_ActivateAbility`
  (`self.ActivationSetUp`)
  (if (`GameplayTagAssetInterface.HasMatchingGameplayTag` (`self.GetAbilitySystemComponentFromActorInfo`) (struct :`TagName` "State.Sprinting"))
    (`AbilityTask_WaitDelay.WaitDelay` 0.03
      (:`OnFinish`
        _))
    (else
      (`GSAT_WaitDelayOneFrame.WaitDelayOneFrame`
        (:`OnFinish`
          _))))
  (`self.BatchRPCTryActivateAbility` (`self.InstantAbilityHandle`) true)
  (`self.K2_EndAbility`))

(fn `ActivationSetUp`
  (`self.SourceWeapon`
    (:`then`
      _)
    (:`else`
      (bind _asgsweapon (cast `GSWeapon` (`self.GetCurrentSourceObject`)))
      (set `self.SourceWeapon` _asgsweapon)))
  (if (not (`GSBlueprintFunctionLibrary.IsAbilitySpecHandleValid` (`self.InstantAbilityHandle`)))
    (bind _asgsability_system_component (cast `GSAbilitySystemComponent` (`self.GetAbilitySystemComponentFromActorInfo`)))
    (set `self.InstantAbilityHandle` (`GSAbilitySystemComponent.FindAbilitySpecHandleForClass` _asgsability_system_component "/Game/Survival/Blueprints/GameplayAbilities/Weapon/Sniper/GA_SniperPrimaryInstant.GA_SniperPrimaryInstant_C" (`self.SourceWeapon`))))
  (`self.InstantAbility`
    (:`then`
      _)
    (:`else`
      (bind _returnvalue (`GSBlueprintFunctionLibrary.GetPrimaryAbilityInstanceFromHandle` (`self.GetAbilitySystemComponentFromActorInfo`) (`self.InstantAbilityHandle`)))
      (bind _asga_sniper_primary_instant (cast `/Game/Survival/Blueprints/GameplayAbilities/Weapon/Sniper/GA_SniperPrimaryInstant` _returnvalue))
      (set `self.InstantAbility` _asga_sniper_primary_instant)))
  (return))

(fn `GSCheckCost`
  (params (Handle :type "GameplayAbilitySpecHandle Structure") (ActorInfo :type "GameplayAbilityActorInfo Structure (by ref)"))
  (returns (ReturnValue :type Boolean))
  (bind (_owneractor _avataractor _playercontroller _abilitysystemcomponent) (break `GameplayAbilityActorInfo` (`local.ActorInfo`)))
  (bind _asgsweapon (cast `GSWeapon` (`self.BP_GetSourceObject` Handle ActorInfo)))
  (if (and (or (>= (`GSWeapon.GetPrimaryClipAmmo` _asgsweapon) (`self.AmmoCost`)) (`GSWeapon.HasInfiniteAmmo` _asgsweapon)) (`parent.GSCheckCost` (`local.Handle`) (`local.ActorInfo`)))
    (return true)
    (else
      (bind _returnvalue (`GSBlueprintFunctionLibrary.IsPrimaryAbilityInstanceActive` _abilitysystemcomponent (`local.Handle`)))
      (if (not _returnvalue)
        (`AbilitySystemComponent.TryActivateAbilitiesByTag` _abilitysystemcomponent (`BlueprintGameplayTagLibrary.MakeGameplayTagContainerFromArray` (`|MakeArray` (struct :`TagName` "Ability.Weapon.Reload") :!type "GameplayTag Structure")) true))
      (return false))))