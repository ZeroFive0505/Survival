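; GA_MagicGunAlternate is the Magic Gun's alternate-fire gameplay ability, toggling the weapon's fire mode between Fire Ball and Ice Ball.
; On activation it lazily caches the GSWeapon from the source object and the GSPlayerController from actor info.
; It switches the FireMode gameplay tag and status text, pushes the text to the player controller's equipped weapon display, then ends.
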(event `self.K2_ActivateAbility`
  (bind (_returnvalue_owneractor _returnvalue_avataractor _returnvalue_playercontroller) (break `GameplayAbilityActorInfo` (`self.GetActorInfo`)))
  (`self.Weapon`
    (:`then`
      (`self.PlayerController` :!label _label
        (:`then`
          _)
        (:`else`
          (bind _asgsplayer_controller (cast `GSPlayerController` _returnvalue_playercontroller))
          (set `self.PlayerController` _asgsplayer_controller)))
      (`|SwitchGameplayTag` (`GSWeapon.FireMode` (`self.Weapon`))
        (:`Weapon.MagicGun.FireMode.FireBall`
          (set `GSWeapon.FireMode` (struct :`TagName` "Weapon.MagicGun.FireMode.IceBall") (`self.Weapon`))
          (set `GSWeapon.StatusText` (`self.IceBallStatus`) (`self.Weapon`)))
        (:`Weapon.MagicGun.FireMode.IceBall`
          (set `GSWeapon.FireMode` (struct :`TagName` "Weapon.MagicGun.FireMode.FireBall") (`self.Weapon`))
          (set `GSWeapon.StatusText` (`self.FireBallStatus`) (`self.Weapon`))))
      (bind _playercontroller (`self.PlayerController`)
        (:`then`
          (`GSPlayerController.SetEquippedWeaponStatusText` _playercontroller (`GSWeapon.StatusText` (`self.Weapon`))))
        (:`else`
          _))
      (`self.K2_EndAbility`))
    (:`else`
      (bind _asgsweapon (cast `GSWeapon` (`self.GetCurrentSourceObject`))
        (:`then`
          (set `self.Weapon` _asgsweapon)
          (goto _label))
        (:`CastFailed`
          (`KismetSystemLibrary.PrintString` "Error: Failed to cast Source Object to GSWeapon" true true (struct :`R` 1.0 :`A` 1.0)))))))