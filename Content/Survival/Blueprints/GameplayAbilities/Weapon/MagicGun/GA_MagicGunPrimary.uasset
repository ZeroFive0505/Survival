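; GA_MagicGunPrimary is the magic gun's primary fire ability, a wrapper that triggers GA_MagicGunPrimaryInstant for each activation.
; It lazily caches the source weapon and the instant ability's spec handle and instance.
; After one frame, or a brief delay when sprinting, it activates and immediately ends the instant ability through a batched RPC.
; On success it commits the cost unless an infinite-ammo tag is present, then ends itself.
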(event `self.K2_ActivateAbility`
  (`self.ActivationSetUp`)
  (if (`GameplayTagAssetInterface.HasMatchingGameplayTag` (`self.GetAbilitySystemComponentFromActorInfo`) (struct :`TagName` "State.Sprinting"))
    (`AbilityTask_WaitDelay.WaitDelay` 0.03
      (:`OnFinish`
        _))
    (else
      (`GSAT_WaitDelayOneFrame.WaitDelayOneFrame`
        (:`OnFinish`
          _))))
  (bind _returnvalue (`self.BatchRPCTryActivateAbility` (`self.InstantAbilityHandle`) true))
  (if _returnvalue
    (if (not (`GameplayTagAssetInterface.HasAnyMatchingGameplayTags` (`AbilitySystemBlueprintLibrary.GetAbilitySystemComponent` (`self.GetAvatarActorFromActorInfo`)) (`self.InfAmmoTag`)))
      (`self.K2_CommitAbilityCost` false)))
  (`self.K2_EndAbility`))

(fn `ActivationSetUp`
  (`self.SourceWeapon`
    (:`then`
      _)
    (:`else`
      (bind _asgsweapon (cast `GSWeapon` (`self.GetCurrentSourceObject`)))
      (set `self.SourceWeapon` _asgsweapon)))
  (if (not (`GSBlueprintFunctionLibrary.IsAbilitySpecHandleValid` (`self.InstantAbilityHandle`)))
    (bind _asgsability_system_component (cast `GSAbilitySystemComponent` (`self.GetAbilitySystemComponentFromActorInfo`)))
    (set `self.InstantAbilityHandle` (`GSAbilitySystemComponent.FindAbilitySpecHandleForClass` _asgsability_system_component "/Game/Survival/Blueprints/GameplayAbilities/Weapon/MagicGun/GA_MagicGunPrimaryInstant.GA_MagicGunPrimaryInstant_C" (`self.SourceWeapon`))))
  (`self.InstantAbility`
    (:`then`
      _)
    (:`else`
      (bind _returnvalue (`GSBlueprintFunctionLibrary.GetPrimaryAbilityInstanceFromHandle` (`self.GetAbilitySystemComponentFromActorInfo`) (`self.InstantAbilityHandle`)))
      (bind _asga_magic_gun_primary_instant (cast `/Game/Survival/Blueprints/GameplayAbilities/Weapon/MagicGun/GA_MagicGunPrimaryInstant` _returnvalue))
      (set `self.InstantAbility` _asga_magic_gun_primary_instant)))
  (return))