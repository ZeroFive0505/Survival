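; Secondary ability of the sci-fi shotgun: hold-to-aim down sights for the survivor.
; Activation applies an aiming effect, tweens first-person FOV and mesh offset, shortens the third-person boom and starts ADS movement.
; Input release applies an aiming-removal effect and tweens back, ending once default FOV is reached.
; OnEndAbility ensures the removal effect was applied, clears both effects and tasks, and snaps camera, mesh and movement back to normal.
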(event `self.K2_ActivateAbility`
  (bind _owningsurvivor (`self.OwningSurvivor`))
  (bind _owningsurvivor_2 (`self.OwningSurvivor`))
  (set `self.GE_AimingRemoval` (struct))
  (`self.OwningSurvivor`
    (:`then`
      _)
    (:`else`
      (bind _asbp_survivor (cast `/Game/Survival/Blueprints/Characters/BP_Survivor` (`self.GetAvatarActorFromActorInfo`)))
      (set `self.OwningSurvivor` _asbp_survivor)))
  (`self.SourceWeapon`
    (:`then`
      _)
    (:`else`
      (bind _asgsweapon (cast `GSWeapon` (`self.GetCurrentSourceObject`)))
      (set `self.SourceWeapon` _asgsweapon)))
  (bind _returnvalue (`self.BP_ApplyGameplayEffectToOwner` (`self.GE_Aiming_Class`) (`self.GetAbilityLevel`)))
  (set `self.GE_Aiming` _returnvalue)
  (bind _asynctaskproxy (`GSAT_WaitChangeFOV.WaitChangeFOV` "None" (`GSSurvivor.FirstPersonCamera` (`self.OwningSurvivor`)) (`self.TargetingFOV`) 0.1)
    (:`then`
      (set `self.ZoomInTask` _asynctaskproxy)
      (set `SpringArmComponent.TargetArmLength` 100.0 (`GSSurvivor.ThirdPersonCameraBoom` (`self.OwningSurvivor`)))
      (`GSAT_MoveSceneCompRelLocation.MoveSceneComponentRelativeLocation` "None" (`GSSurvivor.GetFirstPersonMesh` (`self.OwningSurvivor`)) (- (`SceneComponent.RelativeLocation` (`GSSurvivor.GetFirstPersonMesh` (`self.OwningSurvivor`))) (0.0 0.0 2.5)) 0.1
        (:`then`
          (bind _asgscharacter_movement_component (cast `GSCharacterMovementComponent` (`.MovementComponent` (break `GameplayAbilityActorInfo` (`self.GetActorInfo`)))))
          (`GSCharacterMovementComponent.StartAimDownSights` _asgscharacter_movement_component)
          (`AbilityTask_WaitInputRelease.WaitInputRelease` false
            (:`OnRelease`
              (bind _asynctaskproxy_2 (`GSAT_WaitChangeFOV.WaitChangeFOV` "None" (`GSSurvivor.FirstPersonCamera` _owningsurvivor) (`GSSurvivor.Default1PFOV` _owningsurvivor) 0.05)
                (:`then`
                  (set `self.ZoomResetTask` _asynctaskproxy_2)
                  (bind _returnvalue_2 (`self.BP_ApplyGameplayEffectToOwner` (`self.GE_AimingRemoval_Class`) (`self.GetAbilityLevel`)))
                  (set `self.GE_AimingRemoval` _returnvalue_2)
                  (`GSAT_MoveSceneCompRelLocation.MoveSceneComponentRelativeLocation` "None" (`GSSurvivor.GetFirstPersonMesh` _owningsurvivor_2) (`GSSurvivor.StartingFirstPersonMeshLocation` _owningsurvivor_2) 0.05))
                (:`OnTargetFOVReached`
                  (`self.K2_EndAbility`))))))))))

(event `self.K2_OnEndAbility`
  (params (bWasCancelled :type Boolean))
  (bind _owningsurvivor (`self.OwningSurvivor`))
  (bind _owningsurvivor_2 (`self.OwningSurvivor`))
  (bind _owningsurvivor_3 (`self.OwningSurvivor`))
  (bind _returnvalue (`AbilitySystemBlueprintLibrary.GetActiveGameplayEffectStackCount` (`self.GE_AimingRemoval`)))
  (if (not (> _returnvalue 0))
    (bind _returnvalue_2 (`self.BP_ApplyGameplayEffectToOwner` (`self.GE_AimingRemoval_Class`) (`self.GetAbilityLevel`)))
    (set `self.GE_AimingRemoval` _returnvalue_2))
  (`self.BP_RemoveGameplayEffectFromOwnerWithHandle` (`self.GE_Aiming`))
  (`self.BP_RemoveGameplayEffectFromOwnerWithHandle` (`self.GE_AimingRemoval`))
  (bind _zoomintask (`self.ZoomInTask`)
    (:`then`
      (`GameplayTask.EndTask` _zoomintask))
    (:`else`
      _))
  (bind _zoomresettask (`self.ZoomResetTask`)
    (:`then`
      (`GameplayTask.EndTask` _zoomresettask))
    (:`else`
      _))
  (`CameraComponent.SetFieldOfView` (`GSSurvivor.FirstPersonCamera` _owningsurvivor) (`GSSurvivor.Default1PFOV` _owningsurvivor))
  (set `SpringArmComponent.TargetArmLength` (`GSSurvivor.StartingThirdPersonCameraBoomArmLength` _owningsurvivor_2) (`GSSurvivor.ThirdPersonCameraBoom` _owningsurvivor_2))
  (`SceneComponent.K2_SetRelativeLocation` (`GSSurvivor.GetFirstPersonMesh` _owningsurvivor_3) (`GSSurvivor.StartingFirstPersonMeshLocation` _owningsurvivor_3) false false)
  (bind _asgscharacter_movement_component (cast `GSCharacterMovementComponent` (`.MovementComponent` (break `GameplayAbilityActorInfo` (`self.GetActorInfo`)))))
  (`GSCharacterMovementComponent.StopAimDownSights` _asgscharacter_movement_component))