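; Gameplay ability for the sci-fi shotgun's alternate action, which toggles the weapon between semi-auto and full-auto fire.
; On activation it caches the GSWeapon from the source object and the GSPlayerController from actor info.
; It switches on the weapon's fire mode gameplay tag to swap mode and status text, pushes that text to the player controller, then ends.
; A failed weapon cast only prints an error, leaving the ability un-ended.
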(event `self.K2_ActivateAbility`
  (bind (_returnvalue_owneractor _returnvalue_avataractor _returnvalue_playercontroller) (break `GameplayAbilityActorInfo` (`self.GetActorInfo`)))
  (`self.Weapon`
    (:`then`
      (`self.PlayerController` :!label _label
        (:`then`
          _)
        (:`else`
          (bind _asgsplayer_controller (cast `GSPlayerController` _returnvalue_playercontroller)
            (:`then`
              (set `self.PlayerController` _asgsplayer_controller))
            (:`CastFailed`
              _))))
      (`|SwitchGameplayTag` (`GSWeapon.FireMode` (`self.Weapon`))
        (:`Weapon.Shotgun.FireMode.SemiAuto`
          (set `GSWeapon.FireMode` (struct :`TagName` "Weapon.Shotgun.FireMode.FullAuto") (`self.Weapon`))
          (set `GSWeapon.StatusText` (`self.FullAutoStatus`) (`self.Weapon`)))
        (:`Weapon.Shotgun.FireMode.FullAuto`
          (set `GSWeapon.FireMode` (struct :`TagName` "Weapon.Shotgun.FireMode.SemiAuto") (`self.Weapon`))
          (set `GSWeapon.StatusText` (`self.SemiAutoStatus`) (`self.Weapon`))))
      (bind _playercontroller (`self.PlayerController`)
        (:`then`
          (`GSPlayerController.SetEquippedWeaponStatusText` _playercontroller (`GSWeapon.StatusText` (`self.Weapon`))))
        (:`else`
          _))
      (`self.K2_EndAbility`))
    (:`else`
      (bind _asgsweapon (cast `GSWeapon` (`self.GetCurrentSourceObject`))
        (:`then`
          (set `self.Weapon` _asgsweapon)
          (goto _label))
        (:`CastFailed`
          (`KismetSystemLibrary.PrintString` "Error: Failed to cast Source Object to GSWeapon"))))))