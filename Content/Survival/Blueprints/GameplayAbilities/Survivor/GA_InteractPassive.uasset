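; Passive survivor gameplay ability that detects interactable targets, shows their prompt and description, and triggers interactions on input.
; A target-trace task caches the hit and arms an input wait; a press sends Ability.Interaction with that target once the blocking tag is absent.
; Losing the target cancels pending waits and hides the prompt unless an interaction is active.
; Ability.InteractionEnd re-arms the same targeted component after input release.
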(event `self.K2_ActivateAbility`
  (bind _currenttracedtarget (`self.CurrentTracedTarget`))
  (bind (_returnvalue_bblockinghit _returnvalue_binitialoverlap _returnvalue_time _returnvalue_distance _returnvalue_location _returnvalue_impactpoint _returnvalue_normal _returnvalue_impactnormal _returnvalue_physmat _returnvalue_hitactor _returnvalue_hitcomponent) (`GameplayStatics.BreakHitResult` (`AbilitySystemBlueprintLibrary.GetHitResultFromTargetData` _currenttracedtarget)))
  (bind (_asynctaskproxy _data) (`GSAT_WaitInteractableTarget.WaitForInteractableTarget` "None" (struct :`Name` "InteractTrace") 200.0 0.1 (`self.ShowDebugTrace`))
    (:`then`
      (set `self.WaitForInteractableTargetTask` _asynctaskproxy)
      (bind (_asynctaskproxy_2 _payload) (`AbilityTask_WaitGameplayEvent.WaitGameplayEvent` (struct :`TagName` "Ability.InteractionEnd") null)
        (:`EventReceived`
          (bind (_returnvalue_bblockinghit_2 _returnvalue_binitialoverlap_2 _returnvalue_time_2 _returnvalue_distance_2 _returnvalue_location_2 _returnvalue_impactpoint_2 _returnvalue_normal_2 _returnvalue_impactnormal_2 _returnvalue_physmat_2 _returnvalue_hitactor_2 _returnvalue_hitcomponent_2) (`GameplayStatics.BreakHitResult` (`AbilitySystemBlueprintLibrary.GetHitResultFromTargetData` (`.TargetData` (break `GameplayEventData` _payload)))))
          (if (and (not (`KismetSystemLibrary.IsValid` (`self.WaitInputPressWithTagsTask`))) (not (`KismetSystemLibrary.IsValid` (`self.WaitGameplayTagRemoveTask`))) (== (`AbilitySystemBlueprintLibrary.GetDataCountFromTargetData` (`.TargetData` (break `GameplayEventData` _payload))) 1) (`AbilitySystemBlueprintLibrary.TargetDataHasHitResult` (`.TargetData` (break `GameplayEventData` _payload))) (and (== (`AbilitySystemBlueprintLibrary.GetDataCountFromTargetData` _currenttracedtarget) 1) (`AbilitySystemBlueprintLibrary.TargetDataHasHitResult` _currenttracedtarget)) (== _returnvalue_hitcomponent_2 _returnvalue_hitcomponent))
            (if (`self.IsInputPressed`)
              (bind _asynctaskproxy_3 (`AbilityTask_WaitInputRelease.WaitInputRelease` false)
                (:`then`
                  (set `self.WaitInputReleaseTask` _asynctaskproxy_3))
                (:`OnRelease`
                  (`self.WaitForConfirmation` :!label _label)))
              (else
                (goto _label)))))))
    (:`FoundNewInteractableTarget`
      (set `self.CurrentTracedTarget` _data)
      (`self.WaitForConfirmation`))
    (:`LostInteractableTarget`
      (bind _waitinputpresswithtagstask (`self.WaitInputPressWithTagsTask`)
        (:`then`
          (`GameplayTask.EndTask` _waitinputpresswithtagstask))
        (:`else`
          _))
      (bind _waitgameplaytagremovetask (`self.WaitGameplayTagRemoveTask`)
        (:`then`
          (`GameplayTask.EndTask` _waitgameplaytagremovetask))
        (:`else`
          _))
      (bind _waitinputreleasetask (`self.WaitInputReleaseTask`)
        (:`then`
          (`GameplayTask.EndTask` _waitinputreleasetask))
        (:`else`
          _))
      (`GSBlueprintFunctionLibrary.ClearTargetData` (`self.CurrentTracedTarget`))
      (bind _asgsability_system_component (cast `GSAbilitySystemComponent` (`self.GetAbilitySystemComponentFromActorInfo`)))
      (if (<= (`GSAbilitySystemComponent.BP_GetTagCount` _asgsability_system_component (struct :`TagName` "State.Interacting")) (`GSAbilitySystemComponent.BP_GetTagCount` _asgsability_system_component (struct :`TagName` "State.InteractingRemoval")))
        (bind _asgsplayer_state (cast `GSPlayerState` (`self.GetOwningActorFromActorInfo`)))
        (`GSPlayerState.HideInteractionPrompt` _asgsplayer_state)))))

(event `WaitForConfirmation`
  (bind (_returnvalue_bblockinghit _returnvalue_binitialoverlap _returnvalue_time _returnvalue_distance _returnvalue_location _returnvalue_impactpoint _returnvalue_normal _returnvalue_impactnormal _returnvalue_physmat _returnvalue_hitactor _returnvalue_hitcomponent) (`GameplayStatics.BreakHitResult` (`AbilitySystemBlueprintLibrary.GetHitResultFromTargetData` (`self.CurrentTracedTarget`))))
  (bind _returnvalue (message `GSInteractable.GetInteractionDuration` _returnvalue_hitactor _returnvalue_hitcomponent))
  (bind _returnvalue_2 (message `GSInteractable.GetInteractionDescription` _returnvalue_hitactor _returnvalue_hitcomponent))
  (bind _asgsplayer_state (cast `GSPlayerState` (`self.GetOwningActorFromActorInfo`))
    (:`then`
      (`GSPlayerState.ShowInteractionPrompt` _asgsplayer_state _returnvalue)
      (`GSPlayerState.SetInteractionDescription` _asgsplayer_state _returnvalue_2))
    (:`CastFailed`
      _))
  (bind _asynctaskproxy (`GSAT_WaitInputPressWithTags.WaitInputPressWithTags` (struct) (struct) true)
    (:`then`
      (set `self.WaitInputPressWithTagsTask` _asynctaskproxy))
    (:`OnPress`
      (bind _asynctaskproxy_2 (`AbilityTask_WaitGameplayTagRemoved.WaitGameplayTagRemove` (`self.ActiveBlockedTag`) null true)
        (:`then`
          (set `self.WaitGameplayTagRemoveTask` _asynctaskproxy_2))
        (:`Removed`
          (bind _waitinputpresswithtagstask (`self.WaitInputPressWithTagsTask`)
            (:`then`
              (`GameplayTask.EndTask` _waitinputpresswithtagstask))
            (:`else`
              _))
          (`self.SendGameplayEvent` (struct :`TagName` "Ability.Interaction") (make `GameplayEventData` (struct) null null null null (struct) (struct) (struct) 0.0 (`self.CurrentTracedTarget`))))))))