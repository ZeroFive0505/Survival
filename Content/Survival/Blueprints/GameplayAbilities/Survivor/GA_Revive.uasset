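; Survivor gameplay ability for a revive, played on the avatar that returns to a knocked-down montage if interrupted.
; It scales the revive montage's play rate so the animation lasts exactly the survivor's ReviveDuration, ending the ability on completion.
; A Reviving gameplay effect is applied to the owner as the montage starts and removed by handle when the ability ends.
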(event `self.K2_ActivateAbility`
  (bind _asbp_survivor (cast `/Game/Survival/Blueprints/Characters/BP_Survivor` (`self.GetAvatarActorFromActorInfo`)))
  (`AbilityTask_PlayMontageAndWait.CreatePlayMontageAndWaitProxy` "None" (`self.ReviveMontage`) (/ 1.0 (/ (`GSSurvivor.ReviveDuration` _asbp_survivor) (`AnimationAsset.GetPlayLength` (`self.ReviveMontage`))))
    (:`then`
      (bind _returnvalue (`self.BP_ApplyGameplayEffectToOwner` "/Game/Survival/Blueprints/GameplayEffects/Survivor/GE_Reviving.GE_Reviving_C"))
      (set `self.RevivingHandle` _returnvalue))
    (:`OnCompleted`
      (`self.K2_EndAbility`))))

(event `self.K2_OnEndAbility`
  (params (bWasCancelled :type Boolean))
  (`self.BP_RemoveGameplayEffectFromOwnerWithHandle` (`self.RevivingHandle`))
  (if bWasCancelled
    (`AbilityTask_PlayMontageAndWait.CreatePlayMontageAndWaitProxy` "None" (`self.KnockedDownMontage`))))