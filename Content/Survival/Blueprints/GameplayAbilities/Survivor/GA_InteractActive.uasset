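; Survivor gameplay ability that runs an interaction, instant or held, on an actor component passed in by gameplay event.
; After validating availability and range, it applies GE_Interacting and messages the target through pre/post phases, with optional net syncs around the timed delay.
; Releasing input mid-interaction cancels it; timed interactions stay active until release.
; Ending cleans up effects and timer UI, notifies the target if cancelled, and sends Ability.InteractionEnd.
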(event `self.K2_ActivateAbilityFromEvent`
  (params (EventData :type "GameplayEventData Structure (by ref)"))
  (bind (_returnvalue_bblockinghit _returnvalue_binitialoverlap _returnvalue_time _returnvalue_distance _returnvalue_location _returnvalue_impactpoint _returnvalue_normal _returnvalue_impactnormal _returnvalue_physmat _returnvalue_hitactor _returnvalue_hitcomponent) (`GameplayStatics.BreakHitResult` (`AbilitySystemBlueprintLibrary.GetHitResultFromTargetData` (`self.InteractableTarget`))))
  (bind (_returnvalue_bblockinghit_2 _returnvalue_binitialoverlap_2 _returnvalue_time_2 _returnvalue_distance_2 _returnvalue_location_2 _returnvalue_impactpoint_2 _returnvalue_normal_2 _returnvalue_impactnormal_2 _returnvalue_physmat_2 _returnvalue_hitactor_2 _returnvalue_hitcomponent_2) (`GameplayStatics.BreakHitResult` (`AbilitySystemBlueprintLibrary.GetHitResultFromTargetData` (`self.InteractableTarget`))))
  (bind (_returnvalue_bblockinghit_3 _returnvalue_binitialoverlap_3 _returnvalue_time_3 _returnvalue_distance_3 _returnvalue_location_3 _returnvalue_impactpoint_3 _returnvalue_normal_3 _returnvalue_impactnormal_3 _returnvalue_physmat_3 _returnvalue_hitactor_3 _returnvalue_hitcomponent_3) (`GameplayStatics.BreakHitResult` (`AbilitySystemBlueprintLibrary.GetHitResultFromTargetData` (`self.InteractableTarget`))))
  (bind (_returnvalue_bblockinghit_4 _returnvalue_binitialoverlap_4 _returnvalue_time_4 _returnvalue_distance_4 _returnvalue_location_4 _returnvalue_impactpoint_4 _returnvalue_normal_4 _returnvalue_impactnormal_4 _returnvalue_physmat_4 _returnvalue_hitactor_4 _returnvalue_hitcomponent_4) (`GameplayStatics.BreakHitResult` (`AbilitySystemBlueprintLibrary.GetHitResultFromTargetData` (`self.InteractableTarget`))))
  (bind (_returnvalue_bblockinghit_5 _returnvalue_binitialoverlap_5 _returnvalue_time_5 _returnvalue_distance_5 _returnvalue_location_5 _returnvalue_impactpoint_5 _returnvalue_normal_5 _returnvalue_impactnormal_5 _returnvalue_physmat_5 _returnvalue_hitactor_5 _returnvalue_hitcomponent_5) (`GameplayStatics.BreakHitResult` (`AbilitySystemBlueprintLibrary.GetHitResultFromTargetData` (`self.InteractableTarget`))))
  (bind _isvalid (`self.ValidateTarget` EventData_TargetData))
  (if _isvalid
    (bind _output_get (set `self.InteractableTarget` EventData_TargetData))
    (bind (_returnvalue_bblockinghit_6 _returnvalue_binitialoverlap_6 _returnvalue_time_6 _returnvalue_distance_6 _returnvalue_location_6 _returnvalue_impactpoint_6 _returnvalue_normal_6 _returnvalue_impactnormal_6 _returnvalue_physmat_6 _returnvalue_hitactor_6 _returnvalue_hitcomponent_6) (`GameplayStatics.BreakHitResult` (`AbilitySystemBlueprintLibrary.GetHitResultFromTargetData` _output_get)))
    (bind _returnvalue (message `GSInteractable.GetInteractionDuration` _returnvalue_hitactor_6 _returnvalue_hitcomponent_6))
    (set `self.InteractionDuration` _returnvalue)
    (if (> (`self.InteractionDuration`) 0.0)
      (bind _asynctaskproxy (`AbilityTask_WaitInputRelease.WaitInputRelease` false)
        (:`then`
          (set `self.WaitInputReleaseTask` _asynctaskproxy)
          (set `self.IsInteracting` true :!label _label)
          (bind _returnvalue_2 (`self.BP_ApplyGameplayEffectToOwner` "/Game/Survival/Blueprints/GameplayEffects/Survivor/GE_Interacting.GE_Interacting_C"))
          (set `self.GE_InteractingHandle` _returnvalue_2)
          (message `GSInteractable.RegisterInteracter` _returnvalue_hitactor _returnvalue_hitcomponent (`self.GetAvatarActorFromActorInfo`))
          (bind (_bshouldsync _type) (message `GSInteractable.GetPreInteractSyncType` _returnvalue_hitactor_2 _returnvalue_hitcomponent_2))
          (if _bshouldsync
            (bind _asynctaskproxy_2 (`AbilityTask_NetworkSyncPoint.WaitNetSync` _type)
              (:`then`
                (set `self.PreInteractSyncTask` _asynctaskproxy_2))
              (:`OnSync`
                (message `GSInteractable.PreInteract` _returnvalue_hitactor_3 (`self.GetAvatarActorFromActorInfo`) _returnvalue_hitcomponent_3 :!label _label_2)
                (if (> (`self.InteractionDuration`) 0.0)
                  (bind _asynctaskproxy_3 (`AbilityTask_WaitDelay.WaitDelay` (`self.InteractionDuration`))
                    (:`then`
                      (set `self.WaitDelayTask` _asynctaskproxy_3)
                      (bind _asgsplayer_state (cast `GSPlayerState` (`self.GetOwningActorFromActorInfo`)))
                      (`GSPlayerState.StartInteractionTimer` _asgsplayer_state (`self.InteractionDuration`)))
                    (:`OnFinish`
                      (bind _asgsplayer_state_2 (cast `GSPlayerState` (`self.GetOwningActorFromActorInfo`) :!label _label_3))
                      (`GSPlayerState.StopInteractionTimer` _asgsplayer_state_2)
                      (bind (_bshouldsync_2 _type_2) (message `GSInteractable.GetPostInteractSyncType` _returnvalue_hitactor_4 _returnvalue_hitcomponent_4))
                      (if _bshouldsync_2
                        (bind _asynctaskproxy_4 (`AbilityTask_NetworkSyncPoint.WaitNetSync` _type_2)
                          (:`then`
                            (set `self.PostInteractSyncTask` _asynctaskproxy_4))
                          (:`OnSync`
                            (message `GSInteractable.PostInteract` _returnvalue_hitactor_5 (`self.GetAvatarActorFromActorInfo`) _returnvalue_hitcomponent_5 :!label _label_4)
                            (message `GSInteractable.UnregisterInteracter` _returnvalue_hitactor_5 _returnvalue_hitcomponent_5 (`self.GetAvatarActorFromActorInfo`))
                            (bind _asgsplayer_state_3 (cast `GSPlayerState` (`self.GetOwningActorFromActorInfo`)))
                            (`GSPlayerState.HideInteractionPrompt` _asgsplayer_state_3)
                            (bind _returnvalue_3 (`self.BP_ApplyGameplayEffectToOwner` "/Game/Survival/Blueprints/GameplayEffects/Survivor/GE_InteractingRemoval.GE_InteractingRemoval_C"))
                            (set `self.GE_InteractingRemovalHandle` _returnvalue_3)
                            (`self.BP_RemoveGameplayEffectFromOwnerWithHandle` (`self.GE_InteractingHandle`))
                            (`self.BP_RemoveGameplayEffectFromOwnerWithHandle` (`self.GE_InteractingRemovalHandle`))
                            (set `self.IsInteracting` false)
                            (if (not (> (`self.InteractionDuration`) 0.0))
                              (`self.K2_EndAbility`))))
                        (else
                          (goto _label_4)))))
                  (else
                    (goto _label_3)))))
            (else
              (goto _label_2))))
        (:`OnRelease`
          (if (`self.IsInteracting`)
            (`self.K2_CancelAbility`)
            (else
              (`self.K2_EndAbility`)))))
      (else
        (goto _label)))
    (else
      (`KismetSystemLibrary.PrintString` "Warning: GA_Interact Validate failed")
      (`self.K2_CancelAbility`))))

(event `self.K2_OnEndAbility`
  (params (bWasCancelled :type Boolean))
  (bind _interactabletarget (`self.InteractableTarget`))
  (bind (_returnvalue_bblockinghit _returnvalue_binitialoverlap _returnvalue_time _returnvalue_distance _returnvalue_location _returnvalue_impactpoint _returnvalue_normal _returnvalue_impactnormal _returnvalue_physmat _returnvalue_hitactor _returnvalue_hitcomponent) (`GameplayStatics.BreakHitResult` (`AbilitySystemBlueprintLibrary.GetHitResultFromTargetData` _interactabletarget)))
  (if bWasCancelled
    (if (and (`AbilitySystemBlueprintLibrary.TargetDataHasHitResult` _interactabletarget) (`KismetSystemLibrary.IsValid` _returnvalue_hitactor))
      (message `GSInteractable.CancelInteraction` _returnvalue_hitactor _returnvalue_hitcomponent)))
  (bind _returnvalue (`self.BP_ApplyGameplayEffectToOwner` "/Game/Survival/Blueprints/GameplayEffects/Survivor/GE_InteractingRemoval.GE_InteractingRemoval_C"))
  (set `self.GE_InteractingRemovalHandle` _returnvalue)
  (`self.BP_RemoveGameplayEffectFromOwnerWithHandle` (`self.GE_InteractingHandle`))
  (`self.BP_RemoveGameplayEffectFromOwnerWithHandle` (`self.GE_InteractingRemovalHandle`))
  (bind _asgsplayer_state (cast `GSPlayerState` (`self.GetOwningActorFromActorInfo`)))
  (`GSPlayerState.HideInteractionPrompt` _asgsplayer_state)
  (bind _asgsplayer_state_2 (cast `GSPlayerState` (`self.GetOwningActorFromActorInfo`)))
  (`GSPlayerState.StopInteractionTimer` _asgsplayer_state_2)
  (`self.SendGameplayEvent` (struct :`TagName` "Ability.InteractionEnd") (make `GameplayEventData` (struct) null null null null (struct) (struct) (struct) 0.0 (`self.InteractableTarget`))))

(fn `ValidateTarget`
  (params (TargetData :type "GameplayAbilityTargetDataHandle Structure"))
  (returns (IsValid :type Boolean))
  (bind (_returnvalue_bblockinghit _returnvalue_binitialoverlap _returnvalue_time _returnvalue_distance _returnvalue_location _returnvalue_impactpoint _returnvalue_normal _returnvalue_impactnormal _returnvalue_physmat _returnvalue_hitactor _returnvalue_hitcomponent) (`GameplayStatics.BreakHitResult` (`AbilitySystemBlueprintLibrary.GetHitResultFromTargetData` TargetData)))
  (bind _returnvalue (message `GSInteractable.IsAvailableForInteraction` _returnvalue_hitactor _returnvalue_hitcomponent))
  (return (and _returnvalue (== (`AbilitySystemBlueprintLibrary.GetDataCountFromTargetData` TargetData) 1) (`AbilitySystemBlueprintLibrary.TargetDataHasHitResult` TargetData) (`KismetSystemLibrary.IsValid` _returnvalue_hitactor) (`KismetSystemLibrary.IsValid` _returnvalue_hitcomponent) (<= (`KismetMathLibrary.Vector_DistanceSquared` (`Actor.K2_GetActorLocation` (`self.GetAvatarActorFromActorInfo`)) (`SceneComponent.K2_GetComponentLocation` _returnvalue_hitcomponent)) (`KismetMathLibrary.Square` (`self.MaxDistanceToTarget`))))))