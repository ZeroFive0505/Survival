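; GA_NextWeapon is a survivor gameplay ability that switches to the next weapon.
; It can activate only when the BP_Survivor avatar carries more than one weapon.
; On activation it calls NextWeapon on the survivor, applies the GE_WeaponIsChangingDelayReplicationTag effect to the owner, and ends immediately.
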(event `self.K2_ActivateAbility`
  (bind _asbp_survivor (cast `/Game/Survival/Blueprints/Characters/BP_Survivor` (`self.GetAvatarActorFromActorInfo`)))
  (bind _output_get (set `self.OwningSurvivor` _asbp_survivor))
  (`GSSurvivor.NextWeapon` _output_get)
  (`self.BP_ApplyGameplayEffectToOwner` "/Game/Survival/Blueprints/GameplayEffects/Survivor/GE_WeaponIsChangingDelayReplicationTag.GE_WeaponIsChangingDelayReplicationTag_C")
  (`self.K2_EndAbility`))

(fn `K2_CanActivateAbility`
  (params (ActorInfo :type "GameplayAbilityActorInfo Structure") (Handle :type "GameplayAbilitySpecHandle Structure"))
  (returns (RelevantTags :type "GameplayTagContainer Structure") (ReturnValue :type Boolean))
  (bind _asbp_survivor (cast `/Game/Survival/Blueprints/Characters/BP_Survivor` (`.AvatarActor` (break `GameplayAbilityActorInfo` ActorInfo))))
  (return (struct) (> (`GSSurvivor.GetNumWeapons` _asbp_survivor) 1)))