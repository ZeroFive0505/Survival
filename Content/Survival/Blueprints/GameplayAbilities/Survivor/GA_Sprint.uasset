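; Survivor sprint ability that can activate only while moving roughly toward the view direction.
; It applies a sprinting effect and local cue and starts sprinting on the custom movement component.
; A short delay loop with net sync commits cost while accelerating on the ground.
; Input release, failed cost or a CancelsSprint tag ends it, and OnEndAbility undoes effects, movement and cue.
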(event `self.K2_ActivateAbility`
  (bind (_owneractor _avataractor _playercontroller _abilitysystemcomponent _skeletalmeshcomponent _animinstance _movementcomponent) (break `GameplayAbilityActorInfo` (`self.GetActorInfo`)))
  (set `self.EndSprint` false)
  (bind _returnvalue (`self.BP_ApplyGameplayEffectToOwner` "/Game/Survival/Blueprints/GameplayEffects/Survivor/GE_Sprinting.GE_Sprinting_C"))
  (set `self.SprintingHandle` _returnvalue)
  (bind _asgscharacter_movement_component (cast `GSCharacterMovementComponent` _movementcomponent))
  (`GSCharacterMovementComponent.StartSprinting` _asgscharacter_movement_component)
  (bind _asgsability_system_component (cast `GSAbilitySystemComponent` _abilitysystemcomponent))
  (`GSAbilitySystemComponent.AddGameplayCueLocal` :`self` _asgsability_system_component :`GameplayCueTag` (struct :`TagName` "GameplayCue.Ability.Sprinting"))
  (`AbilityTask_WaitInputRelease.WaitInputRelease` true
    (:`then`
      (bind _asynctaskproxy (`AbilityTask_WaitGameplayTagAdded.WaitGameplayTagAdd` (struct :`TagName` "Ability.CancelsSprint") null true)
        (:`then`
          (set `self.WaitCancelsSprintTagAddedTask` _asynctaskproxy)
          (`AbilityTask_WaitDelay.WaitDelay` 0.05 :!label _label
            (:`OnFinish`
              (`AbilityTask_NetworkSyncPoint.WaitNetSync` "OnlyServerWait"
                (:`OnSync`
                  (bind _asgscharacter_movement_component_2 (cast `GSCharacterMovementComponent` (`.MovementComponent` (break `GameplayAbilityActorInfo` (`self.GetActorInfo`)))))
                  (if (and (> (`KismetMathLibrary.VSize` (`CharacterMovementComponent.GetCurrentAcceleration` _asgscharacter_movement_component_2)) 0.0) (not (`NavMovementComponent.IsFalling` _asgscharacter_movement_component_2)))
                    (bind _returnvalue_2 (`self.K2_CommitAbilityCost` false))
                    (if _returnvalue_2
                      (if (not (`self.EndSprint`)) :!label _label_2
                        (goto _label))
                      (else
                        (set `self.EndSprint` true :!label _label_3)
                        (`self.K2_EndAbility`)))
                    (else
                      (goto _label_2))))))))
        (:`Added`
          (`AbilityTask_NetworkSyncPoint.WaitNetSync` "OnlyServerWait"
            (:`OnSync`
              (goto _label_3))))))
    (:`OnRelease`
      (goto _label_3))))

(event `self.K2_OnEndAbility`
  (params (bWasCancelled :type Boolean))
  (bind (_owneractor _avataractor _playercontroller _abilitysystemcomponent _skeletalmeshcomponent _animinstance _movementcomponent) (break `GameplayAbilityActorInfo` (`self.GetActorInfo`)))
  (bind _returnvalue (`self.BP_ApplyGameplayEffectToOwner` "/Game/Survival/Blueprints/GameplayEffects/Survivor/GE_SprintingRemoval.GE_SprintingRemoval_C"))
  (set `self.SprintingRemovalHandle` _returnvalue)
  (`self.BP_RemoveGameplayEffectFromOwnerWithHandle` (`self.SprintingHandle`))
  (`self.BP_RemoveGameplayEffectFromOwnerWithHandle` (`self.SprintingRemovalHandle`))
  (bind _asgscharacter_movement_component (cast `GSCharacterMovementComponent` _movementcomponent)
    (:`then`
      (`GSCharacterMovementComponent.StopSprinting` _asgscharacter_movement_component))
    (:`CastFailed`
      _))
  (bind _waitcancelssprinttagaddedtask (`self.WaitCancelsSprintTagAddedTask`)
    (:`then`
      (`GameplayTask.EndTask` _waitcancelssprinttagaddedtask))
    (:`else`
      _))
  (bind _asgsability_system_component (cast `GSAbilitySystemComponent` _abilitysystemcomponent))
  (`GSAbilitySystemComponent.RemoveGameplayCueLocal` :`self` _asgsability_system_component :`GameplayCueTag` (struct :`TagName` "GameplayCue.Ability.Sprinting")))

(fn `K2_CanActivateAbility`
  (params (ActorInfo :type "GameplayAbilityActorInfo Structure") (Handle :type "GameplayAbilitySpecHandle Structure"))
  (returns (RelevantTags :type "GameplayTagContainer Structure") (ReturnValue :type Boolean))
  (bind (_owneractor _avataractor _playercontroller) (break `GameplayAbilityActorInfo` ActorInfo))
  (bind _returnvalue (`Actor.GetVelocity` _avataractor))
  (return (struct) (and (> (`KismetMathLibrary.VSize` _returnvalue) 0.0) (>= (`KismetMathLibrary.Dot_VectorVector` (`KismetMathLibrary.Normal` _returnvalue) (`KismetMathLibrary.GetForwardVector` (`Controller.GetControlRotation` _playercontroller))) 0.5))))