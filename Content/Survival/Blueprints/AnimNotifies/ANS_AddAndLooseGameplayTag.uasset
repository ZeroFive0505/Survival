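; Anim notify state that grants loose gameplay tags to a GSCharacter for the duration of a window in an animation.
; Notify begin casts the mesh owner to GSCharacter, gets its GSAbilitySystemComponent and adds the configured GameplayTags.
; Notify end repeats the lookup and removes the same tags.
; Both events do nothing to the tags if either cast fails.
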(fn `Received_NotifyBegin`
  (params (MeshComp :type "SkeletalMeshComponent Object Reference") (Animation :type "AnimSequenceBase Object Reference") (TotalDuration :type "Float (single-precision)") (EventReference :type "AnimNotifyEventReference Structure (by ref)"))
  (returns (ReturnValue :type Boolean))
  (bind _asgscharacter (cast `GSCharacter` (`ActorComponent.GetOwner` MeshComp)))
  (bind _asgsability_system_component (cast `GSAbilitySystemComponent` (`AbilitySystemBlueprintLibrary.GetAbilitySystemComponent` _asgscharacter)))
  (`GSAbilitySystemComponent.BP_AddLooseGameplayTags` _asgsability_system_component (`self.GameplayTags`) 1)
  (return true))

(fn `Received_NotifyEnd`
  (params (MeshComp :type "SkeletalMeshComponent Object Reference") (Animation :type "AnimSequenceBase Object Reference") (EventReference :type "AnimNotifyEventReference Structure (by ref)"))
  (returns (ReturnValue :type Boolean))
  (bind _asgscharacter (cast `GSCharacter` (`ActorComponent.GetOwner` MeshComp)))
  (bind _asgsability_system_component (cast `GSAbilitySystemComponent` (`AbilitySystemBlueprintLibrary.GetAbilitySystemComponent` _asgscharacter)))
  (`GSAbilitySystemComponent.BP_RemoveLooseGameplayTags` _asgsability_system_component (`self.GameplayTags`) 1)
  (return true))