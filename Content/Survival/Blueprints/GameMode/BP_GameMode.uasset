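; Survival game mode that runs randomized enemy waves with possible mid-wave ambushes.
; EnemySpawn staggers spawns across random spawn points, while SpawnAmbush uses a looping timer at ambush points, both feeding a remaining-enemy count.
; Enemy deaths roll against AmbushRatio for one ambush per wave, or at zero remaining show a countdown and build the next shuffled wave.
; BeginPlay is empty, leaving the spawn-point lookup and first-wave setup disconnected.
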(event `self.ReceiveBeginPlay`)

(event `EnemySpawn`
  (bind _spawnpoints (`self.SpawnPoints`))
  (bind _returnvalue_location (`KismetMathLibrary.BreakTransform` (`self.GetTransform` (`|GetArrayItem` _spawnpoints (`KismetMathLibrary.RandomInteger` (`KismetArrayLibrary.Array_Length` _spawnpoints))))))
  (set `self.RemainingEnemies` (+ (`self.RemainingEnemies`) (`KismetArrayLibrary.Array_Length` (`self.EnemiesToSpawn`))))
  (set `self.CurrentIndex` 0)
  (bind _returnvalue (`|SpawnActorFromClass` (`|GetArrayItem` (`self.EnemiesToSpawn`) (`self.CurrentIndex`)) (`KismetMathLibrary.MakeTransform` _returnvalue_location) "AlwaysSpawn" "MultiplyWithRoot" null null :!label _label))
  (add `self.OnDestroyed` _returnvalue (`|CreateDelegate` :!event `EnemyOnDestroyed`))
  (`/Engine/EditorBlueprintResources/StandardMacros.IncrementInt` (`self.CurrentIndex`)
    (:`  `
      (`KismetSystemLibrary.Delay` (`KismetMathLibrary.RandomFloatInRange` 1.0 5.0))
      (if (< (`self.CurrentIndex`) (`KismetArrayLibrary.Array_Length` (`self.EnemiesToSpawn`)))
        (goto _label)))))

(event `SpawnAmbush`
  (params (EnemiesToSpawn :type Integer))
  (set `self.RemainingEnemies` (+ (`self.RemainingEnemies`) EnemiesToSpawn))
  (set `self.AmbushEnemies` EnemiesToSpawn)
  (set `self.AmbushCount` 0)
  (bind _returnvalue (`KismetSystemLibrary.K2_SetTimerDelegate` (`|CreateDelegate` :!event `AmbushSpawnTimer`) (`KismetMathLibrary.RandomFloatInRange` 1.5 3.0) true))
  (set `self.AmbushHandle` _returnvalue))

(event `AmbushSpawnTimer`
  (bind _enemiestospawn (`self.EnemiesToSpawn`))
  (bind _ambushpoints (`self.AmbushPoints`))
  (bind _returnvalue_location (`KismetMathLibrary.BreakTransform` (`self.GetTransform` (`|GetArrayItem` _ambushpoints (`KismetMathLibrary.RandomInteger` (`KismetArrayLibrary.Array_Length` _ambushpoints))))))
  (bind _result (`/Engine/EditorBlueprintResources/StandardMacros.IncrementInt` (`self.AmbushCount`))
    (:`  `
      (if (> _result (`self.AmbushEnemies`))
        (if (`KismetSystemLibrary.K2_IsValidTimerHandle` (`self.AmbushHandle`))
          (`KismetSystemLibrary.K2_ClearAndInvalidateTimerHandle` (`self.AmbushHandle`)))
        (else
          (bind _returnvalue (`|SpawnActorFromClass` (`|GetArrayItem` _enemiestospawn (`KismetMathLibrary.RandomInteger` (`KismetArrayLibrary.Array_Length` _enemiestospawn))) (`KismetMathLibrary.MakeTransform` _returnvalue_location) "AlwaysSpawn" "MultiplyWithRoot" null null))
          (add `self.OnDestroyed` _returnvalue (`|CreateDelegate` :!event `EnemyOnDestroyed`)))))))

(event `EnemyOnDestroyed` :!signature `self.OnDestroyed`
  (params (DestroyedActor :type "Actor Object Reference"))
  (bind _enemyvariety (`self.EnemyVariety`))
  (bind _result (`/Engine/EditorBlueprintResources/StandardMacros.DecrementInt` (`self.RemainingEnemies`))
    (:`  `
      (if (<= _result 0)
        (`KismetArrayLibrary.Array_Clear` (`self.EnemiesToSpawn`))
        (`self.WaveFinish`)
        (bind _returnvalue (`|CreateWidget` "/Game/Survival/Blueprints/UI/WBP_PrepareNextWave.WBP_PrepareNextWave_C" null "Prepare for the Next Wave.."))
        (`UserWidget.AddToViewport` _returnvalue 10)
        (`KismetSystemLibrary.Delay` 15.0)
        (bind _asbp_controller (cast `/Game/Survival/Blueprints/Controller/BP_Controller` (`GameplayStatics.GetPlayerController` 0)))
        (`GSHUDWidget.SetRespawnCountdown` (`GSPlayerController.UIHUDWidget` _asbp_controller) 5.0)
        (`KismetSystemLibrary.Delay` 5.0)
        (`KismetArrayLibrary.Array_Shuffle` (`self.EnemyVariety`))
        (for _ (range (+ (`KismetMathLibrary.Clamp` (`KismetMathLibrary.RandomInteger` 16) 5 15) 1))
          (`KismetArrayLibrary.Array_Add` (`self.EnemiesToSpawn`) (`|GetArrayItem` _enemyvariety (`KismetMathLibrary.RandomInteger` (`KismetArrayLibrary.Array_Length` _enemyvariety)))))
        (`Widget.RemoveFromParent` _returnvalue)
        (`self.EnemySpawn`)
        (goto _label_2 :!via `Reset`)
        (elif (<= (`KismetMathLibrary.RandomFloat`) (`self.AmbushRatio`))
          (`/Engine/EditorBlueprintResources/StandardMacros.DoOnce` false :!label _label_2
            (:`Completed`
              (`self.SpawnAmbush` (`KismetMathLibrary.Clamp` (`KismetMathLibrary.RandomInteger` 11) 5 10))
              (bind _returnvalue_2 (`|CreateWidget` "/Game/Survival/Blueprints/UI/WBP_PrepareNextWave.WBP_PrepareNextWave_C" null "Enemy Ambush!!"))
              (`UserWidget.AddToViewport` _returnvalue_2 10)
              (`KismetSystemLibrary.Delay` 5.0)
              (`Widget.RemoveFromParent` _returnvalue_2))))))))

(fn `UserConstructionScript`)