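; BP_Goblin is a goblin enemy that fights in melee and can drop loot.
; On BeginPlay it spawns a random weapon class and attaches it to the mesh's WeaponSocket.
; Melee attacks activate GA_GoblinMelee through the Ability System, while the ranged attack is an empty stub.
; When destroyed it removes the weapon and, by DropRatio chance, spawns a random item from DropItems.
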(event `self.ReceiveBeginPlay`
  (bind _weapon (`self.Weapon`))
  (bind _returnvalue (`|SpawnActorFromClass` (`|GetArrayItem` _weapon (`KismetMathLibrary.RandomInteger` (`KismetArrayLibrary.Array_Length` _weapon))) (`KismetMathLibrary.MakeTransform` (0.0 0.0 0.0)) "AlwaysSpawn" "MultiplyWithRoot" self self self))
  (bind _output_get (set `self.WeaponActor` _returnvalue))
  (`self.K2_AttachToComponent` _output_get (`self.Mesh`) "WeaponSocket" "SnapToTarget" "SnapToTarget" "SnapToTarget" false))

(event `self.ApplyForceAtBone`
  (params (BoneName :type Name) (ForceAmount :type "Float (single-precision)") (Direction :type "Vector Structure"))
  (`PrimitiveComponent.AddForce` (`self.Mesh`) (* Direction ForceAmount) BoneName true))

(event `DoMeleeAttack`
  (`AbilitySystemComponent.TryActivateAbilityByClass` (`AbilitySystemBlueprintLibrary.GetAbilitySystemComponent` self) "/Game/Survival/Blueprints/GameplayAbilities/Enemy/Goblin/GA_GoblinMelee.GA_GoblinMelee_C" true))

(event `self.ReceiveDestroyed`
  (bind _dropitems (`self.DropItems`))
  (`|ExecutionSequence`
    (:`then_0`
      (if (<= (`KismetMathLibrary.RandomFloat`) (`self.DropRatio`))
        (`KismetArrayLibrary.Array_Shuffle` _dropitems)
        (`|SpawnActorFromClass` (`|GetArrayItem` _dropitems (`KismetMathLibrary.RandomInteger` (`KismetArrayLibrary.Array_Length` _dropitems))) (`KismetMathLibrary.MakeTransform` (+ (`SceneComponent.K2_GetComponentLocation` (`self.Mesh`)) (0.0 0.0 50.0))) "AlwaysSpawn" "MultiplyWithRoot" null null)))
    (:`then_1`
      (`self.K2_DestroyActor` (`self.WeaponActor`)))))

(event `DoRangeAttack`)

(fn `GetHeadBoneName`
  (returns (ReturnValue :type Name))
  (return "b_MF_Head"))

(fn `UserConstructionScript`)