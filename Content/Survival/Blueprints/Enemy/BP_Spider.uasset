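; Spider enemy Blueprint that carries its own weapon and drops loot when destroyed.
; On BeginPlay it spawns a BP_SpiderWeapon and attaches it to the front right knee socket of its mesh.
; On destruction it makes chance-based drops of random items at nearby navigable points, then destroys the weapon.
; It also applies acceleration-based force to named bones and reports "head" as its head bone.
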(event `self.ReceiveBeginPlay`
  (bind _returnvalue (`|SpawnActorFromClass` "/Game/Survival/Blueprints/Weapon/Enemy/BP_SpiderWeapon.BP_SpiderWeapon_C" (`KismetMathLibrary.MakeTransform` (0.0 0.0 0.0)) "Undefined" "MultiplyWithRoot" self self self))
  (bind _output_get (set `self.WeaponActor` _returnvalue))
  (`self.K2_AttachToComponent` _output_get (`self.Mesh`) "Front_Right_Knee" "SnapToTarget" "SnapToTarget" "SnapToTarget" true))

(event `self.ApplyForceAtBone`
  (params (BoneName :type Name) (ForceAmount :type "Float (single-precision)") (Direction :type "Vector Structure"))
  (`PrimitiveComponent.AddForce` (`self.Mesh`) (* Direction ForceAmount) BoneName true))

(event `self.ReceiveDestroyed`
  (bind _dropitems (`self.DropItems`))
  (`|ExecutionSequence`
    (:`then_0`
      (`KismetArrayLibrary.Array_Shuffle` (`self.DropItems`))
      (for _ (range (+ (`self.DropItemCount`) 1))
        (if (<= (`KismetMathLibrary.RandomFloat`) (`self.DropRate`))
          (bind _randomlocation (`NavigationSystemV1.K2_GetRandomLocationInNavigableRadius` (`SceneComponent.K2_GetComponentLocation` (`self.Mesh`)) 300.0 null null))
          (`|SpawnActorFromClass` (`|GetArrayItem` _dropitems (`KismetMathLibrary.RandomInteger` (`KismetArrayLibrary.Array_Length` _dropitems))) (`KismetMathLibrary.MakeTransform` (+ _randomlocation (0.0 0.0 50.0))) "AlwaysSpawn" "MultiplyWithRoot" null null))))
    (:`then_1`
      (`self.K2_DestroyActor` (`self.WeaponActor`)))))

(fn `GetHeadBoneName`
  (returns (ReturnValue :type Name))
  (return "head"))

(fn `UserConstructionScript`)