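; BP_Zombie is a survival-game enemy character that attacks in melee and can drop loot.
; On BeginPlay it spawns a BP_ZombieWeapon attached to its mesh, and it triggers melee attacks through the GA_ZombieMelee gameplay ability.
; Death stops its audio, while destruction removes the weapon and rolls DropRatio to spawn a random DropItems entry.
; It also supplies its head bone name and applies directional forces to mesh bones.
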(event `self.ReceiveBeginPlay`
  (bind _returnvalue (`|SpawnActorFromClass` "/Game/Survival/Blueprints/Weapon/Enemy/BP_ZombieWeapon.BP_ZombieWeapon_C" (`KismetMathLibrary.MakeTransform` (0.0 0.0 0.0)) "Undefined" "MultiplyWithRoot" null self self))
  (bind _output_get (set `self.Weapon` _returnvalue))
  (`self.K2_AttachToComponent` _output_get (`self.Mesh`) "None" "SnapToTarget" "SnapToTarget" "SnapToTarget" true)
  (add `self.OnCharacterDied` (delegate `OnCharacterDied_Event`)))

(event `OnCharacterDied_Event` :!signature `self.OnCharacterDied`
  (params (Character :type "GSCharacter Object Reference"))
  (`AudioComponent.Stop` (`self.Audio`)))

(event `self.ReceiveDestroyed`
  (bind _dropitems (`self.DropItems`))
  (`|ExecutionSequence`
    (:`then_0`
      (if (<= (`KismetMathLibrary.RandomFloat`) (`self.DropRatio`))
        (`KismetArrayLibrary.Array_Shuffle` (`self.DropItems`))
        (`|SpawnActorFromClass` (`|GetArrayItem` _dropitems (`KismetMathLibrary.RandomInteger` (`KismetArrayLibrary.Array_Length` _dropitems))) (`KismetMathLibrary.MakeTransform` (`SceneComponent.K2_GetComponentLocation` (`self.Mesh`))) "AlwaysSpawn" "MultiplyWithRoot" null null)))
    (:`then_1`
      (`self.K2_DestroyActor` (`self.Weapon`)))))

(event `DoMeleeAttack`
  (`AbilitySystemComponent.TryActivateAbilityByClass` (`AbilitySystemBlueprintLibrary.GetAbilitySystemComponent` null) "/Game/Survival/Blueprints/GameplayAbilities/Enemy/Zombie/GA_ZombieMelee.GA_ZombieMelee_C" true))

(event `self.ApplyForceAtBone`
  (params (BoneName :type Name) (ForceAmount :type "Float (single-precision)") (Direction :type "Vector Structure"))
  (`PrimitiveComponent.AddForce` (`self.Mesh`) (* Direction ForceAmount) BoneName true))

(fn `GetHeadBoneName`
  (returns (ReturnValue :type Name))
  (return "head"))

(fn `UserConstructionScript`)